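; Laser emitter puzzle actor that fires a straight beam and notifies whatever it hits.
; While IsActive, Tick line-traces on the Visibility channel from the LaserDirection component along its forward vector up to LaserDistance.
; On a hit, it draws the beam as a debug line and sends hit location, normal and incoming direction to actors implementing BPI_LaserInteraction.
; The beam visual relies solely on debug drawing, including the trace's own ForDuration display.
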(event `self.ReceiveBeginPlay`)

(event `self.ReceiveTick`
  (params (DeltaSeconds :type "Float (single-precision)"))
  (bind _laserdirection (`self.LaserDirection`))
  (bind _returnvalue (`SceneComponent.GetForwardVector` _laserdirection))
  (bind _returnvalue_2 (`SceneComponent.K2_GetComponentLocation` _laserdirection))
  (if (`self.bIsActive`)
    (bind (_outhit _returnvalue_3) (`KismetSystemLibrary.LineTraceSingle` :`Start` _returnvalue_2 :`End` (+ _returnvalue_2 (* _returnvalue (`self.LaserDistance`))) :`TraceChannel` (enumliteral `ETraceTypeQuery` "TraceTypeQuery1") :`DrawDebugType` (enumliteral `EDrawDebugTrace` "ForDuration") :`DrawTime` 0.0))
    (if _returnvalue_3
      (bind (_bblockinghit _binitialoverlap _time _distance _location _impactpoint _normal _impactnormal _physmat _hitactor) (`GameplayStatics.BreakHitResult` _outhit))
      (`KismetSystemLibrary.DrawDebugLine` _returnvalue_2 _impactpoint (`self.LaserColor`) 0.0 (`self.LaserThickness`))
      (if (`KismetSystemLibrary.DoesImplementInterface` _hitactor "/Game/Puzzles/BPI_LaserInteraction.BPI_LaserInteraction_C")
        (message `/Game/Puzzles/BPI_LaserInteraction.OnLaserHit` _hitactor _impactpoint _impactnormal (`KismetMathLibrary.Normal` _returnvalue))))))

(event `self.ReceiveActorBeginOverlap`
  (params (OtherActor :type "Actor Object Reference")))

(fn `UserConstructionScript`)