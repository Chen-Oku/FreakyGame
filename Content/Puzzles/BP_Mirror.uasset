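; Puzzle mirror that reflects lasers and can be rotated through interaction.
; LaserUpdate bounces front-side hits about the surface normal, line-traces onward, draws the beam with debug lines and relays the hit through BPI_LaserInteraction, allowing chained reflections.
; StartInteract offsets the target yaw by RotationAngle when CanRotate is set.
; Tick interpolates toward that target, stopping once the interpolated yaw reaches or exceeds it.
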(event `/Game/Puzzles/BPI_LaserInteraction.LaserUpdate`
  (params (HitLocation :type "Vector Structure") (HitNormal :type "Vector Structure") (IncomingDirection :type "Vector Structure"))
  (bind _returnvalue (`KismetMathLibrary.MirrorVectorByNormal` IncomingDirection HitNormal))
  (if (< (`KismetMathLibrary.Dot_VectorVector` (`self.GetActorForwardVector`) IncomingDirection) 0.0)
    (bind (_outhit _returnvalue_2) (`KismetSystemLibrary.LineTraceSingle` :`Start` HitLocation :`End` (+ HitLocation (* _returnvalue 10000.0)) :`TraceChannel` "TraceTypeQuery1" :`DrawDebugType` "ForDuration" :`DrawTime` 0.0))
    (if _returnvalue_2
      (bind (_bblockinghit _binitialoverlap _time _distance _location _impactpoint _normal _impactnormal _physmat _hitactor) (`GameplayStatics.BreakHitResult` _outhit))
      (`KismetSystemLibrary.DrawDebugLine` HitLocation _impactpoint (struct :`R` 1.0 :`G` 1.0 :`A` 1.0) 0.0 5.0)
      (if (`KismetSystemLibrary.DoesImplementInterface` _hitactor "/Game/Puzzles/BPI_LaserInteraction.BPI_LaserInteraction_C")
        (message `/Game/Puzzles/BPI_LaserInteraction.LaserUpdate` _hitactor _impactpoint _impactnormal _returnvalue)))))

(event `/Game/Blueprints/LaserMiniGame/BPI_FreakInteract.StartInteract`
  (if (`self.bCanRotate`)
    (set `self.TargetRotation` (`KismetMathLibrary.MakeRotator` (.roll (`self.K2_GetActorRotation`)) (.pitch (`self.K2_GetActorRotation`)) (+ (.yaw (`self.K2_GetActorRotation`)) (`self.RotationAngle`))))
    (set `self.bIsRotating` true)))

(event `self.ReceiveTick`
  (params (DeltaSeconds :type "Float (single-precision)"))
  (bind _targetrotation (`self.TargetRotation`))
  (bind _returnvalue (`KismetMathLibrary.RInterpTo` (`self.K2_GetActorRotation`) _targetrotation DeltaSeconds (`self.RotationSpeed`)))
  (if (`self.bIsRotating`)
    (`self.K2_SetActorRotation` _returnvalue)
    (if (<= 0.0 (- (.yaw _returnvalue) (.yaw _targetrotation)))
      (set `self.bIsRotating` false))))

(fn `UserConstructionScript`)