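; Laser receiver puzzle Blueprint that activates a linked door once it accumulates enough laser exposure.
; Each LaserUpdate event adds a fixed time step, independent of delta time, to a running total that nothing here resets.
; On reaching the required time, it latches as activated and sends an activation message to Door if valid.
; A redundant ConnectedDoor self-assignment follows, and the debug print is disconnected.
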(event `/Game/Puzzles/BPI_LaserInteraction.LaserUpdate`
  (params (HitLocation :type "Vector Structure") (HitNormal :type "Vector Structure") (IncomingDirection :type "Vector Structure"))
  (bind _door (`self.Door`))
  (bind _output_get (set `self.CurrentLaserTime` (+ (`self.CurrentLaserTime`) 0.016)))
  (if (>= _output_get (`self.RequiredLaserTime`))
    (if (not (`self.bIsActivated`))
      (set `self.bIsActivated` true)
      (`/Engine/EditorBlueprintResources/StandardMacros.IsValid` _door
        (:`Is Valid`
          (message `/Game/Puzzles/BPI_LaserInteraction.OnReceiverActivated` _door)
          (set `self.Connected Door` (`self.ConnectedDoor`)))))))

(fn `UserConstructionScript`)