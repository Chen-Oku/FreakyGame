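; Two-sided tug-of-war rope minigame actor where each interact input pulls the flag (Bandera) its way.
; Each press adds to that side's counter, shakes the camera and timeline-lerps the flag, while Tick moves the camera along with it.
; StartGame resets state and takes over the view without splitscreen.
; Reaching LimiteVictoria triggers a delayed EndGame that notifies both start platforms, activates spawner lasers and restores the shared camera.
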(event `self.ReceiveTick`
  (params (DeltaSeconds :type "Float (single-precision)"))
  (bind _camera (`self.Camera`))
  (bind (_relativelocation_x _relativelocation_y _relativelocation_z) (`KismetMathLibrary.BreakVector` (`SceneComponent.RelativeLocation` _camera)))
  (`SceneComponent.K2_SetRelativeLocation` _camera (`KismetMathLibrary.MakeVector` (+ (- (.x (`SceneComponent.RelativeLocation` (`self.Bandera`))) (`self.NewVarBanderaXInicial`)) 244.716587) _relativelocation_y _relativelocation_z) false false))

(event `self.ReceiveBeginPlay`
  (bind _returnvalue (`GameplayStatics.GetPlayerController` 0))
  (bind _bandera (`self.Bandera`))
  (set `self.NewVarBanderaXInicial` (.x (`SceneComponent.RelativeLocation` (`self.Bandera`))))
  (set `self.PosicionInicial` (`SceneComponent.RelativeLocation` _bandera))
  (set `self.Direccion` (`SceneComponent.GetForwardVector` _bandera))
  (`self.EnableInput` _returnvalue)
  (`EnhancedInputSubsystemInterface.AddMappingContext` (pcsubsystem `EnhancedInputLocalPlayerSubsystem` _returnvalue) null 0 (struct)))

(event `EnhancedInput|/Game/Input/FreakyInputs/Actions/IA_FreakInteract`
  (params (ActionValue :type Boolean) (ElapsedSeconds :type "Float (double-precision)") (TriggeredSeconds :type "Float (double-precision)") (InputAction :type "InputAction Object Reference" :default "/Game/Input/FreakyInputs/Actions/IA_FreakInteract.IA_FreakInteract"))
  ; Game
  (:`Triggered`
    (if (`self.EmpezarJuego`)
      (if (not (`self.JuegoTerminado`))
        (`PlayerCameraManager.StartCameraShake` :`self` (`GameplayStatics.GetPlayerCameraManager` 0) :`ShakeClass` "/Game/Blueprints/SharedCamera/CS_CamareRope.CS_CamareRope_C")
        (set `self.Contador_C` (+ (`self.Contador_C`) 1))
        (bind _output_get (set `self.PosicionObjetivo` (- (`self.PosicionObjetivo`) 4.0)))
        (if (>= (`self.Contador_C`) (`self.LimiteVictoria`))
          (set `self.JuegoTerminado` true)
          (`self.EndGame`)
          (set `self.PosicionObjetivo` -200.0)
          (bind (_direction _suav) (`Timeline|Suav` :!via `PlayFromStart` :!label _label)
            (:`Update`
              (`SceneComponent.K2_SetRelativeLocation` (`self.Bandera`) (`KismetMathLibrary.VLerp` (`SceneComponent.RelativeLocation` (`self.Bandera`)) (`KismetMathLibrary.MakeVector` (`self.PosicionObjetivo`)) _suav) false false)))
          (else
            (goto _label :!via `PlayFromStart`)))))))

(event `/Game/Blueprints/MiniGames/BP_StartGameInterface.StartGame`
  (params (Player1 :type Integer) (Player2 :type Integer))
  (`SceneComponent.K2_SetRelativeLocation` (`self.Bandera`) (`self.PosicionInicial`) false false)
  (`|ExecutionSequence`
    (:`then_0`
      (bind _returnvalue (`GameplayStatics.GetActorOfClass` "/Game/Blueprints/MiniGames/BP_StartMinigameB1.BP_StartMinigameB1_C"))
      (`/Game/Blueprints/MiniGames/BP_StartMinigameB1.EndGamePlatform` _returnvalue false))
    (:`then_1`
      (bind _returnvalue_2 (`GameplayStatics.GetActorOfClass` "/Game/Blueprints/MiniGames/BP_StartMinigameB2.BP_StartMinigameB2_C"))
      (`/Game/Blueprints/MiniGames/BP_StartMinigameB2.EndGamePlatform` _returnvalue_2 false))
    (:`then_2`
      (`/Game/Blueprints/Interabable_Object/BPL_GlobalFunctions.Change Camera` false)
      (`GameplayStatics.SetForceDisableSplitscreen` true)
      (`PlayerController.SetViewTargetWithBlend` (`GameplayStatics.GetPlayerController` 0) self 0.0 "VTBlend_Linear" 0.0 false))
    (:`then_3`
      (set `self.Contador_C` 0)
      (set `self.Contador_M` 0)
      (set `self.JuegoTerminado` false)
      (set `self.PosicionObjetivo` 0.0)
      (set `self.EmpezarJuego` true))))

(event `EnhancedInput|/Game/Input/FreakyInputs/Actions/IA_FreakInteract1`
  (params (ActionValue :type Boolean) (ElapsedSeconds :type "Float (double-precision)") (TriggeredSeconds :type "Float (double-precision)") (InputAction :type "InputAction Object Reference" :default "/Game/Input/FreakyInputs/Actions/IA_FreakInteract1.IA_FreakInteract1"))
  ; Game
  (:`Triggered`
    (if (`self.EmpezarJuego`)
      (if (not (`self.JuegoTerminado`))
        (`PlayerCameraManager.StartCameraShake` :`self` (`GameplayStatics.GetPlayerCameraManager` 0) :`ShakeClass` "/Game/Blueprints/SharedCamera/CS_CamareRope.CS_CamareRope_C")
        (set `self.Contador_M` (+ (`self.Contador_M`) 1))
        (bind _output_get (set `self.PosicionObjetivo` (- (`self.PosicionObjetivo`) -4.0)))
        (if (>= (`self.Contador_M`) (`self.LimiteVictoria`))
          (set `self.JuegoTerminado` true)
          (`self.EndGame`)
          (set `self.PosicionObjetivo` 200.0)
          (bind (_direction _suav) (`Timeline|Cronograma` :!via `PlayFromStart` :!label _label_2)
            (:`Update`
              (`SceneComponent.K2_SetRelativeLocation` (`self.Bandera`) (`KismetMathLibrary.VLerp` (`SceneComponent.RelativeLocation` (`self.Bandera`)) (`KismetMathLibrary.MakeVector` (`self.PosicionObjetivo`)) _suav) false false)))
          (else
            (goto _label_2 :!via `PlayFromStart`)))))))

(event `EndGame`
  ; Game
  (`KismetSystemLibrary.Delay` 5.0)
  (`/Game/Blueprints/Interabable_Object/BPL_GlobalFunctions.Change Camera` true)
  (`KismetSystemLibrary.Delay` 1.0)
  (bind _returnvalue (`GameplayStatics.GetActorOfClass` "/Game/Blueprints/MiniGames/BP_StartMinigameB1.BP_StartMinigameB1_C"))
  (`/Game/Blueprints/MiniGames/BP_StartMinigameB1.EndGamePlatform` _returnvalue true)
  (bind _returnvalue_2 (`GameplayStatics.GetActorOfClass` "/Game/Blueprints/MiniGames/BP_StartMinigameB2.BP_StartMinigameB2_C"))
  (`/Game/Blueprints/MiniGames/BP_StartMinigameB2.EndGamePlatform` _returnvalue_2 true)
  (bind _outactors (`GameplayStatics.GetAllActorsOfClass` "/Game/Blueprints/LaserMiniGame/LaserGameV3/Blueprints/BP_Spawn2.BP_Spawn2_C"))
  (for _array_element _outactors
    (`/Game/Blueprints/LaserMiniGame/LaserGameV3/Blueprints/BuildingBlocks/BPS_Emitter.ActivateLaser` (`/Game/Blueprints/LaserMiniGame/LaserGameV3/Blueprints/BP_Spawn2.BPS_Emitter` _array_element))
    (bind _returnvalue_3 (`GameplayStatics.GetActorOfClass` "/Game/Blueprints/SharedCamera/BP_SharedSplitCamera.BP_SharedSplitCamera_C"))
    (`/Game/Blueprints/SharedCamera/BP_SharedSplitCamera.RestoreSharedCamera` _returnvalue_3)))

(fn `UserConstructionScript`)