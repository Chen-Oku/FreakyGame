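; Blueprint function library of small global helpers for input prompts, camera and effects.
; It looks up the display name of the first key mapped to an Enhanced Input action through the player's local subsystem.
; It also finds the BP_SharedSplitCamera actor and passes player camera data to its MGCamera function.
; A third helper activates or deactivates a particle system from a visibility flag.
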(fn `Activate/Deactivate Particles`
  (params (IsVisible :type Boolean) (ParticleSystem :type "NiagaraComponent Object Reference"))
  (if IsVisible
    (`ActorComponent.Activate` ParticleSystem false)
    (else
      (`ActorComponent.Deactivate` ParticleSystem))))

(fn `Change Camera`
  (params (PlayersCam :type Boolean))
  (bind _returnvalue (`GameplayStatics.GetActorOfClass` null "/Game/Blueprints/SharedCamera/BP_SharedSplitCamera.BP_SharedSplitCamera_C"))
  (`/Game/Blueprints/MiniGames/BP_StartGameInterface.MGCamera` _returnvalue PlayersCam))

(fn `Get Binding Key`
  (params (PlayerController :type "PlayerController Object Reference") (Action :type "InputAction Object Reference"))
  (returns (ReturnValue :type Text))
  (return (`KismetInputLibrary.Key_GetDisplayName` (`|GetArrayItem` (`EnhancedInputSubsystemInterface.QueryKeysMappedToAction` (pcsubsystem `EnhancedInputLocalPlayerSubsystem` PlayerController) Action)))))