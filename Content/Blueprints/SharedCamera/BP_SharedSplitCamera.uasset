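; Shared two-player camera that merges the view when players are close and switches to split screen when they separate.
; A fast looping timer moves it to the players' midpoint and interpolates spring arm length from their clamped separation.
; A slower timer, gated by PlayersCam, compares distance to a fixed threshold, toggling forced splitscreen disable, view target and HUD layout.
; Characters register as player references, and RestoreSharedCamera reapplies view target and HUD.
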(event `MoveCamera`
  (bind _springarm (`self.SpringArm`))
  (bind _playerone (`self.PlayerOne`)
    (:`then`
      (bind _playertwo (`self.PlayerTwo`)
        (:`then`
          (set `SpringArmComponent.TargetArmLength` (`KismetMathLibrary.FInterpTo` (`SpringArmComponent.TargetArmLength` _springarm) (`KismetMathLibrary.FClamp` (`self.GetDistanceTo` _playerone _playertwo) (`self.MinArmLength`) (`self.MaxArmLength`)) (`KismetSystemLibrary.GetGameTimeInSeconds`) (`self.InterpSpeed`)) _springarm)
          (bind _output_get (set `self.AvgPlayerDistance` (`KismetMathLibrary.VLerp` (`self.K2_GetActorLocation` (`self.PlayerOne`)) (`self.K2_GetActorLocation` (`self.PlayerTwo`)) 0.5)))
          (`self.K2_SetActorLocation` self _output_get true false))
        (:`else`)))
    (:`else`)))

(event `self.ReceiveBeginPlay`
  (`KismetSystemLibrary.K2_SetTimer` null "CheckPlayerDistance" 1.0 true)
  (`KismetSystemLibrary.K2_SetTimer` null "MoveCamera" 0.01 true))

(event `CheckPlayerDistance`
  (bind _returnvalue (`GameplayStatics.GetPlayerController` 0))
  (bind _bissplitscreen (`self.bIsSplitScreen`))
  (bind _playerone (`self.PlayerOne`))
  (if (`self.Players Cam`)
    (bind _playerone_2 (`self.PlayerOne`)
      (:`then`
        (bind _playertwo (`self.PlayerTwo`)
          (:`then`
            (bind _returnvalue_2 (< (`self.GetDistanceTo` _playerone_2 _playertwo) 1300.0))
            (`GameplayStatics.SetForceDisableSplitscreen` _returnvalue_2)
            (if _returnvalue_2
              (if _bissplitscreen
                (set `self.bIsSplitScreen` false)
                (`PlayerController.SetViewTargetWithBlend` _returnvalue self 0.0 "VTBlend_Linear" 0.0 false)
                (`/Game/Blueprints/PlayerZD/BP_PlayerCharacterZD.SwitchHUDToFullscreen` _playerone)
                (`/Game/Blueprints/PlayerZD/BP_PlayerCharacterZD.SwitchHUDToFullscreen` (`self.PlayerTwo`)))
              (elif (not _bissplitscreen)
                (set `self.bIsSplitScreen` true)
                (`PlayerController.SetViewTargetWithBlend` _returnvalue _playerone_2 0.0 "VTBlend_Linear" 0.0 false)
                (`/Game/Blueprints/PlayerZD/BP_PlayerCharacterZD.SwitchHUDToSplitScreen` _playerone)
                (`/Game/Blueprints/PlayerZD/BP_PlayerCharacterZD.SwitchHUDToSplitScreen` (`self.PlayerTwo`)))))
          (:`else`)))
      (:`else`))))

(event `RestoreSharedCamera`
  (bind _returnvalue (`GameplayStatics.GetPlayerController` 0))
  (bind _playerone (`self.PlayerOne`))
  (`PlayerController.SetViewTargetWithBlend` _returnvalue (`self.PlayerOne`) 0.0 "VTBlend_Linear" 0.0 false)
  (`PlayerController.SetViewTargetWithBlend` _returnvalue self 0.0 "VTBlend_Linear" 0.0 false)
  (if (`self.bIsSplitScreen`)
    (`/Game/Blueprints/PlayerZD/BP_PlayerCharacterZD.SwitchHUDToSplitScreen` _playerone)
    (`/Game/Blueprints/PlayerZD/BP_PlayerCharacterZD.SwitchHUDToSplitScreen` (`self.PlayerTwo`))
    (else
      (`/Game/Blueprints/PlayerZD/BP_PlayerCharacterZD.SwitchHUDToFullscreen` _playerone)
      (`/Game/Blueprints/PlayerZD/BP_PlayerCharacterZD.SwitchHUDToFullscreen` (`self.PlayerTwo`)))))

(event `MakePlayerReference`
  (params (CharacterRef :type "/Game/Blueprints/PlayerZD/BP_PlayerCharacterZD Object Reference"))
  (`self.PlayerOne`
    (:`then`
      (set `self.PlayerTwo` CharacterRef))
    (:`else`
      (set `self.PlayerOne` CharacterRef))))

(event `/Game/Blueprints/MiniGames/BP_StartGameInterface.MGCamera`
  (params (PlayersCam :type Boolean))
  (set `self.Players Cam` PlayersCam))

(fn `UserConstructionScript`)