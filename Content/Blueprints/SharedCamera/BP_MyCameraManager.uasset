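; Shared two-player camera actor that switches between a single shared view and split-screen based on player distance.
; Characters register through MakePlayerRef, and a fast timer moves the actor to their midpoint while interpolating spring arm length from their clamped separation.
; A slower timer disables split-screen and targets this camera when players are close, otherwise returning player 0's view to PlayerOne.
; TriggerCamShake plays world camera shakes.
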(event `MoveCamera`
  (bind _springarm (`self.SpringArm`))
  (bind _playerone (`self.PlayerOne`)
    (:`then`
      (bind _playertwo (`self.PlayerTwo`)
        (:`then`
          (set `SpringArmComponent.TargetArmLength` (`KismetMathLibrary.FInterpTo` (`SpringArmComponent.TargetArmLength` _springarm) (`KismetMathLibrary.FClamp` (`self.GetDistanceTo` _playerone _playertwo) (`self.MinArmLength`) (`self.MaxArmLength`)) (`KismetSystemLibrary.GetGameTimeInSeconds`) (`self.InterpSpeed`)) _springarm)
          (bind _output_get (set `self.AvgPlayerDistance` (`KismetMathLibrary.VLerp` (`self.K2_GetActorLocation` (`self.PlayerOne`)) (`self.K2_GetActorLocation` (`self.PlayerTwo`)) 0.5)))
          (`self.K2_SetActorLocation` self _output_get true false))
        (:`else`)))
    (:`else`)))

(event `self.ReceiveBeginPlay`
  (`KismetSystemLibrary.K2_SetTimer` null "CheckPlayerDistance" 1.0 true)
  (`KismetSystemLibrary.K2_SetTimer` null "MoveCamera" 0.01 true))

(event `CheckPlayerDistance`
  (bind _returnvalue (`GameplayStatics.GetPlayerController` 0))
  (bind _playerone (`self.PlayerOne`)
    (:`then`
      (bind _playertwo (`self.PlayerTwo`)
        (:`then`
          (bind _returnvalue_2 (< (`self.GetDistanceTo` _playerone _playertwo) 1300.0))
          (`GameplayStatics.SetForceDisableSplitscreen` _returnvalue_2)
          (if _returnvalue_2
            (`PlayerController.SetViewTargetWithBlend` _returnvalue self 0.0 "VTBlend_Linear" 0.0 false)
            (else
              (`PlayerController.SetViewTargetWithBlend` _returnvalue _playerone 0.0 "VTBlend_Linear" 0.0 false))))
        (:`else`)))
    (:`else`)))

(event `MakePlayerRef`
  (params (CharacterRef :type "/Game/Blueprints/PlayerZD/BP_PlayerCharacterZD Object Reference"))
  (`self.PlayerOne`
    (:`then`
      (set `self.PlayerTwo` CharacterRef))
    (:`else`
      (set `self.PlayerOne` CharacterRef))))

(fn `TriggerCamShake`
  (params (ShakeEffect :type "CameraShakeBase Class Reference") (Epicenter :type "Vector Structure") (OuterRadius :type "Float (double-precision)"))
  (`GameplayStatics.PlayWorldCameraShake` ShakeEffect Epicenter 0.0 OuterRadius))

(fn `UserConstructionScript`)