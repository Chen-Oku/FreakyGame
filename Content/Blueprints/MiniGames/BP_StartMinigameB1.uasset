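; Start platform for a two-player minigame that lets a player ready up and starts the Rope game once both are waiting.
; A sphere tracks which player is inside, and interacting toggles the waiting state and calls that player's movement event.
; Per-player timelines tint a dynamic base material and update start particles.
; SetSecondPlayer receives the other player's state, and when both wait, the Rope actor gets StartGameMessage.
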(event `self.Sphere.OnComponentBeginOverlap`
  (params (OverlappedComponent :type "PrimitiveComponent Object Reference") (OtherActor :type "Actor Object Reference") (OtherComp :type "PrimitiveComponent Object Reference") (OtherBodyIndex :type Integer) (bFromSweep :type Boolean) (SweepResult :type "HitResult Structure (by ref)"))
  ; Player Detection
  (if (== OtherActor (`/Game/Blueprints/MiniGames/BP_VariablesManager.P1` (`self.GM_Vars`)))
    (set `self.P1In` true)
    (elif (`self.ActorHasTag` OtherActor "Player2")
      (set `self.P2In` true))))

(event `self.Sphere.OnComponentEndOverlap`
  (params (OverlappedComponent :type "PrimitiveComponent Object Reference") (OtherActor :type "Actor Object Reference") (OtherComp :type "PrimitiveComponent Object Reference") (OtherBodyIndex :type Integer))
  ; Player Detection
  (if (== OtherActor (`/Game/Blueprints/MiniGames/BP_VariablesManager.P1` (`self.GM_Vars`)))
    (set `self.P1In` false)
    (elif (`self.ActorHasTag` OtherActor "Player2")
      (set `self.P2In` false))))

(event `self.ReceiveBeginPlay`
  (bind _returnvalue (`PrimitiveComponent.CreateDynamicMaterialInstance` (`self.Base`) 0 "/Game/Blueprints/MiniGames/M_StartMinigameBase.M_StartMinigameBase" "None"))
  (set `self.MaterialColor` _returnvalue)
  (bind _returnvalue_2 (`GameplayStatics.GetActorOfClass` "/Game/Blueprints/MiniGames/BP_VariablesManager.BP_VariablesManager_C"))
  (set `self.GM_Vars` _returnvalue_2)
  (`/Game/Blueprints/Interabable_Object/BPL_GlobalFunctions.Activate/Deactivate Particles` false (`self.NS_StartParticles`) (`self.NS_StartParticlesEmpty`)))

(event `self.StartInteract`
  ; Inputs
  (if (`self.ToggleInteract`) :!label _label
    (if (`self.P1In`)
      (if (`self.WaitFirstPlayer`)
        (if (== false (`/Game/Blueprints/PlayerZD/BP_PlayerCharacterZD.CanMoveP1` (`/Game/Blueprints/MiniGames/BP_VariablesManager.P1` (`self.GM_Vars`))))
          (`/Game/Blueprints/PlayerZD/BP_PlayerCharacterZD.CanMoveP1Event` (`/Game/Blueprints/MiniGames/BP_VariablesManager.P1` (`self.GM_Vars`)))
          (set `self.WaitFirstPlayer` false)
          (if (`self.WaitFirstPlayer`) :!label _label_2
            (bind (_direction _color) (`Timeline|ChangeColor` :!label _label_3)
              (:`Update`
                (`MaterialInstanceDynamic.SetVectorParameterValue` (`self.MaterialColor`) "Base Color" _color)
                (set `self.Player 1` 0)
                (`/Game/Blueprints/Interabable_Object/BPL_GlobalFunctions.Activate/Deactivate Particles` (`self.WaitFirstPlayer`) (`self.NS_StartParticles`) (`self.NS_StartParticlesEmpty`) :!label _label_4)
                (if (and (== (`self.WaitFirstPlayer`) true) (== (`self.WaitSecondPlayer`) true)) :!label _label_5
                  (bind _returnvalue (`GameplayStatics.GetActorOfClass` "/Game/Blueprints/Rope/Rope.Rope_C"))
                  (message `/Game/Blueprints/MiniGames/BP_StartGameInterface.StartGame` _returnvalue 0 0))))
            (else
              (goto _label_3 :!via `Reverse`))))
        (else
          (`/Game/Blueprints/PlayerZD/BP_PlayerCharacterZD.CanMoveP1Event` (`/Game/Blueprints/MiniGames/BP_VariablesManager.P1` (`self.GM_Vars`)))
          (set `self.WaitFirstPlayer` true)
          (goto _label_2)))
      (elif (`self.P2In`)
        (if (`self.WaitFirstPlayer`)
          (if (== false (`/Game/Blueprints/PlayerZD/BP_PlayerCharacterZD.CanMoveP2` (`/Game/Blueprints/MiniGames/BP_VariablesManager.P1` (`self.GM_Vars`))))
            (`/Game/Blueprints/PlayerZD/BP_PlayerCharacterZD.CanMoveP2Event` (`/Game/Blueprints/MiniGames/BP_VariablesManager.P1` (`self.GM_Vars`)))
            (set `self.WaitFirstPlayer` false)
            (if (`self.WaitFirstPlayer`) :!label _label_6
              (bind (_direction_2 _color_2) (`Timeline|Timeline` :!label _label_7)
                (:`Update`
                  (`MaterialInstanceDynamic.SetVectorParameterValue` (`self.MaterialColor`) "Base Color" _color_2)
                  (set `self.Player 1` 1)
                  (goto _label_4)))
              (else
                (goto _label_7 :!via `Reverse`))))
          (else
            (`/Game/Blueprints/PlayerZD/BP_PlayerCharacterZD.CanMoveP2Event` (`/Game/Blueprints/MiniGames/BP_VariablesManager.P1` (`self.GM_Vars`)))
            (set `self.WaitFirstPlayer` true)
            (goto _label_6)))))))

(event `self.ReceiveTick`
  (params (DeltaSeconds :type "Float (single-precision)")))

(event `EndGamePlatform`
  (params (ToggleInteract :type Boolean))
  ; Inputs
  (set `self.ToggleInteract` ToggleInteract)
  (goto _label))

(event `/Game/Blueprints/MiniGames/BP_StartGameInterface.SetSecondPlayer`
  (params (Player :type Integer) (WaitSecondPlayer :type Boolean))
  (set `self.Player 2` Player)
  (set `self.WaitSecondPlayer` WaitSecondPlayer)
  (goto _label_5))

(fn `EdGraph_5`
  (params (Mole :type Integer :default 0) (Wait :type Boolean :default false))
  (returns (NewParam :type Boolean))
  (return false))

(fn `PlayPushAnim`
  (returns (TrueIfAnim :type Boolean))
  (return false))

(fn `UserConstructionScript`)