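; BP_PauseManager is an actor that toggles the game's pause menu with the Tab key.
; It enables input from player controller 0 on BeginPlay and tracks the current state in the EstaPausado flag.
; Pausing creates a new WBP_PauseMenu widget, adds it to the viewport, pauses the game and shows the cursor.
; Unpausing removes the stored widget, resumes the game and hides the cursor.
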(event `Key|Tab` :paused true
  (params (Key :type "Key Structure"))
  (bind _returnvalue (`GameplayStatics.GetPlayerController` 0))
  (:`Pressed`
    (if (`self.EstaPausado`)
      (`Widget.RemoveFromParent` (`self.PauseMenuRef`))
      (`GameplayStatics.SetGamePaused` false)
      (set `PlayerController.bShowMouseCursor` false _returnvalue)
      (set `self.EstaPausado` false)
      (else
        (bind _returnvalue_2 (`|CreateWidget` "/Game/Blueprints/MenuPausa/WBP_PauseMenu.WBP_PauseMenu_C"))
        (bind _output_get (set `self.PauseMenuRef` _returnvalue_2))
        (`UserWidget.AddToViewport` _output_get 0)
        (`GameplayStatics.SetGamePaused` true)
        (set `PlayerController.bShowMouseCursor` true _returnvalue)
        (set `self.EstaPausado` true)))))

(event `self.ReceiveBeginPlay`
  (`self.EnableInput` (`GameplayStatics.GetPlayerController` 0)))

(fn `UserConstructionScript`)