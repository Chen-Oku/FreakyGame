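; Laser minigame mirror that reflects an incoming beam and can optionally be rotated by the player.
; LaserUpdate checks the beam faces the mirror's front, reflects it by the surface normal, line-traces onward and updates Niagara beam and bounce effects.
; It messages the hit actor with one fewer bounce, forming a chain that LaserStop shuts down through the last hit actor.
; StartInteract uses a timeline to rotate by a fixed pitch or yaw step.
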(event `self.LaserUpdate`
  (params (HitLocation :type "Vector Structure") (HitNormal :type "Vector Structure") (IncomingDirection :type "Vector Structure") (BouncesRemain :type Integer) (SourceActor :type "Actor Object Reference"))
  (bind _bounces_remain (`self.Bounces Remain`))
  (bind _ns_lightbounce (`self.NS_LightBounce`))
  (bind (_endbeam _incomingdircalculated) (`self.BeamBounceDir` (`self.Hit Current Location`) (`self.Hit Normal`) (`self.Incoming Direction`)))
  (if (not (== SourceActor self))
    ; CalculoLaser
    (if (`self.IsActive?`)
      (set `self.Hit Current Location` HitLocation)
      (set `self.Hit Normal` HitNormal)
      (set `self.Incoming Direction` IncomingDirection)
      (set `self.Bounces Remain` BouncesRemain)
      (if (> (`self.Bounces Remain`) 1)
        (if (< (`KismetMathLibrary.Dot_VectorVector` (`self.GetActorForwardVector`) (`self.Incoming Direction`)) 0.0)
          (`|ExecutionSequence`
            (:`then_0`
              ;; Niagara Viz Update
              (`self.UpdateBeamViz` (`self.Hit Current Location`)))
            (:`then_1`
              (set `self.Incoming Dir Calculated` _incomingdircalculated)
              (bind (_outhit _returnvalue) (`KismetSystemLibrary.LineTraceSingle` :`Start` (`self.Hit Current Location`) :`End` _endbeam :`TraceChannel` "TraceTypeQuery1" :`DrawTime` 0.0))
              (bind (_bblockinghit _binitialoverlap _time _distance _location _impactpoint _normal _impactnormal _physmat _hitactor _hitcomponent _hitbonename _bonename _hititem _elementindex _faceindex _tracestart _traceend) (`GameplayStatics.BreakHitResult` _outhit))
              (bind _returnvalue_2 (`KismetMathLibrary.SelectVector` _impactpoint _traceend _bblockinghit))
              (`FXSystemComponent.SetVectorParameter` (`self.NS_Beam`) "BeamEnd" _returnvalue_2 :!label _label)
              (`ActorComponent.Activate` _ns_lightbounce false)
              (`SceneComponent.K2_SetWorldLocation` _ns_lightbounce _returnvalue_2 false false)
              (if _returnvalue
                (if true
                  (if (!= _hitactor (`self.LastHitMirror`))
                    (`self.LastHitMirror` :!label _label_2
                      (:`then`
                        (`/Game/Blueprints/LaserMiniGame/MirrorMiniGame/BPI_LaserInteraction.LaserStop` null)
                        (set `self.IsActive?` true))
                      (:`else`
                        _))
                    (set `self.LastHitMirror` _hitactor)
                    (if (<= _bounces_remain 0)
                      (`/Game/Blueprints/LaserMiniGame/MirrorMiniGame/BPI_LaserInteraction.LaserStop` null)
                      (set `self.IsActive?` true)
                      (else
                        (message `/Game/Blueprints/LaserMiniGame/MirrorMiniGame/BPI_LaserInteraction.LaserUpdate` _hitactor _impactpoint _impactnormal (`self.Incoming Dir Calculated`) (- _bounces_remain 1) self :!label _label_3)))
                    (else
                      (goto _label_3)))
                  (else
                    (goto _label_2)))
                (else
                  (goto _label_2)))))
          (else
            (goto _label)))))))

(event `self.LaserStop`
  (params (SourceActor :type "Actor Object Reference"))
  (bind _ns_lightbounce (`self.NS_LightBounce`))
  (bind _ns_beam (`self.NS_Beam`))
  (bind _lasthitmirror (`self.LastHitMirror`))
  (`ActorComponent.Deactivate` _ns_beam)
  (`SceneComponent.SetVisibility` _ns_beam false false)
  (`ActorComponent.Deactivate` _ns_lightbounce)
  (`SceneComponent.SetVisibility` _ns_lightbounce false false)
  (`/Engine/EditorBlueprintResources/StandardMacros.IsValid` _lasthitmirror
    (:`Is Valid`
      (message `/Game/Blueprints/LaserMiniGame/MirrorMiniGame/BPI_LaserInteraction.LaserStop` _lasthitmirror SourceActor)
      (set `self.LastHitMirror` null))))

(event `self.StartInteract`
  (bind _returnvalue (`self.K2_GetActorRotation`))
  ; Interact and H/V-Rotation
  (if (and (`self.bCanRotate`) (not (`self.bIsRotating`)))
    (bind _output_get (set `self.InicialRotation` _returnvalue))
    (if (`self.bVerticalRotation`)
      (set `self.TargetRotation` (`KismetMathLibrary.ComposeRotators` _returnvalue (`KismetMathLibrary.MakeRotator` 0.0 (`self.VertRotationAngle`))))
      (else
        (bind _output_get_2 (set `self.TargetRotation` (`KismetMathLibrary.ComposeRotators` _returnvalue (`KismetMathLibrary.MakeRotator` 0.0 0.0 (`self.HorRotationAngle`)))))))
    (set `self.bIsRotating` true)
    (bind (_direction _rotacionanim) (`Timeline|Timeline_0` :`NewTime` 5.0 :!via `PlayFromStart`)
      (:`Update`
        (`self.K2_SetActorRotation` (`KismetMathLibrary.RLerp` _output_get _output_get_2 _rotacionanim true)))
      (:`Finished`
        (set `self.bIsRotating` false)))))

(fn `BeamBounceDir`
  (params (HitActorVec :type "Vector Structure") (InNormal :type "Vector Structure") (InVect :type "Vector Structure"))
  (returns (EndBeam :type "Vector Structure") (IncomingDirCalculated :type "Vector Structure"))
  (bind _returnvalue (`KismetMathLibrary.MirrorVectorByNormal` InVect InNormal))
  (return (+ HitActorVec (* _returnvalue 10000.0)) _returnvalue))

(fn `CanReceiveLaser?`
  (returns (bCanReceive :type Boolean))
  (return true))

(fn `UpdateBeamViz`
  (params (Param :type "Vector Structure"))
  (`ActorComponent.Activate` (`self.NS_LightBounce`) false)
  (`ActorComponent.Activate` (`self.NS_Beam`) true)
  (`SceneComponent.SetVisibility` (`self.NS_LightBounce`) true false)
  (`SceneComponent.SetVisibility` (`self.NS_Beam`) true false)
  (`FXSystemComponent.SetVectorParameter` (`self.NS_Beam`) "Beam Start" Param))

(fn `UserConstructionScript`)