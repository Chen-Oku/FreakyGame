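; Laser emitter for the mirror minigame that fires a beam from its LaserDirection component.
; While active, a fast looping timer line-traces forward, stretching a Niagara beam and moving a bounce effect to the hit point or trace end.
; It sends the hit actor interface messages carrying direction and remaining bounces, and tells the previous mirror to stop when the target changes.
; The emitter itself cannot receive lasers.
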(event `self.ReceiveBeginPlay`
  (`self.LaserEmitter`))

(event `LaserEmitter`
  (`KismetSystemLibrary.K2_SetTimer` null "UpdateLaser" 0.001 true))

(event `UpdateLaser`
  (bind _ns_lightbounce (`self.NS_LightBounce`))
  (bind _lastmirror (`self.LastMirror`))
  (bind _laserdirection (`self.LaserDirection`))
  (bind _returnvalue (`SceneComponent.GetForwardVector` _laserdirection))
  (bind _returnvalue_2 (`SceneComponent.K2_GetComponentLocation` _laserdirection))
  (if (`self.bIsActive`)
    (`FXSystemComponent.SetVectorParameter` (`self.NS_Beam`) "Beam Start" _returnvalue_2)
    (bind (_outhit _returnvalue_3) (`KismetSystemLibrary.LineTraceSingle` :`Start` _returnvalue_2 :`End` (+ _returnvalue_2 (* _returnvalue (`self.LaserDistance`))) :`TraceChannel` (enumliteral `ETraceTypeQuery` "TraceTypeQuery1") :`DrawDebugType` (enumliteral `EDrawDebugTrace` "ForDuration") :`DrawTime` 0.0))
    (bind (_bblockinghit _binitialoverlap _time _distance _location _impactpoint _normal _impactnormal _physmat _hitactor _hitcomponent _hitbonename _bonename _hititem _elementindex _faceindex _tracestart _traceend) (`GameplayStatics.BreakHitResult` _outhit))
    (bind _returnvalue_4 (`KismetMathLibrary.SelectVector` _impactpoint _traceend _bblockinghit))
    (`FXSystemComponent.SetVectorParameter` (`self.NS_Beam`) "BeamEnd" _returnvalue_4)
    (`ActorComponent.Activate` _ns_lightbounce false)
    (`SceneComponent.K2_SetWorldLocation` _ns_lightbounce _returnvalue_4 false false)
    (if _returnvalue_3
      (bind _bcanreceive (message `/Game/Blueprints/LaserMiniGame/MirrorMiniGame/BPI_LaserInteraction.CanReceiveLaser?` _hitactor))
      (if _bcanreceive
        (if (!= _hitactor _lastmirror)
          (`/Engine/EditorBlueprintResources/StandardMacros.IsValid` _lastmirror :!label _label
            (:`Is Valid`
              (message `/Game/Blueprints/LaserMiniGame/MirrorMiniGame/BPI_LaserInteraction.LaserStop` _lastmirror null :!label _label_2)
              (set `self.LastMirror` _hitactor))
            (:`Is Not Valid`
              (set `self.LastMirror` _hitactor))))
        (else
          (goto _label_2)))
      (else
        (goto _label)))
    (message `/Game/Blueprints/LaserMiniGame/MirrorMiniGame/BPI_LaserInteraction.LaserUpdate` _hitactor _impactpoint _impactnormal (`KismetMathLibrary.Normal` _returnvalue) 5 self _)))

(event `/Game/Blueprints/LaserMiniGame/MirrorMiniGame/BPI_LaserInteraction.LaserStop`
  (params (SourceActor :type "Actor Object Reference"))
  (bind _lastmirror (`self.LastMirror`))
  (if (not (== SourceActor self))
    (`ActorComponent.Deactivate` (`self.NS_Beam`))
    (`SceneComponent.SetVisibility` (`self.NS_Beam`) false false)
    (`/Engine/EditorBlueprintResources/StandardMacros.IsValid` _lastmirror
      (:`Is Valid`
        (set `self.LastMirror` null)
        (message `/Game/Blueprints/LaserMiniGame/MirrorMiniGame/BPI_LaserInteraction.LaserStop` _lastmirror null)))))

(fn `CanReceiveLaser?`
  (returns (bCanReceive :type Boolean))
  (return false))

(fn `UserConstructionScript`)