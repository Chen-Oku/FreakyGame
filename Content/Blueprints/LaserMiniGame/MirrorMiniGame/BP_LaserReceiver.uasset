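; BP_LaserReceiver is a laser target in the mirror minigame that notifies a door after enough laser exposure.
; LaserUpdate accumulates delta time until the required duration, checks CanReceiveLaser (always true here), then activates once and messages a valid Door before clearing ConnectedDoor.
; LaserStop resets the timer and activation flag, without sending the door any message.
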(event `/Game/Blueprints/LaserMiniGame/MirrorMiniGame/BPI_LaserInteraction.LaserUpdate`
  (params (HitLocation :type "Vector Structure") (HitNormal :type "Vector Structure") (IncomingDirection :type "Vector Structure") (BouncesRemain :type Integer))
  (bind _door (`self.Door`))
  (bind _output_get (set `self.CurrentLaserTime` (+ (`self.CurrentLaserTime`) (`GameplayStatics.GetWorldDeltaSeconds`))))
  (if (>= _output_get (`self.RequiredLaserTime`))
    (bind _bcanreceive (`/Game/Blueprints/LaserMiniGame/MirrorMiniGame/BPI_LaserInteraction.CanReceiveLaser?`))
    (if _bcanreceive
      (if (not (`self.bIsActivated`))
        (set `self.bIsActivated` true)
        (`/Engine/EditorBlueprintResources/StandardMacros.IsValid` _door
          (:`Is Valid`
            (message `/Game/Blueprints/LaserMiniGame/MirrorMiniGame/BPI_LaserInteraction.OnReceiverActivated` _door)
            (set `self.Connected Door` null)))))))

(event `/Game/Blueprints/LaserMiniGame/MirrorMiniGame/BPI_LaserInteraction.LaserStop`
  (set `self.CurrentLaserTime` 0.0)
  (set `self.bIsActivated` false))

(fn `CanReceiveLaser?`
  (returns (bCanReceive :type Boolean))
  (return true))

(fn `UserConstructionScript`)