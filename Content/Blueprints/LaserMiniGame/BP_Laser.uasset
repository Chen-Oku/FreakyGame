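; Laser emitter for the laser minigame that rotates a 45-degree yaw step each time it is interacted with.
; A Visibility line trace from the arrow sets the beam length, scaling the cylinder mesh to the hit distance or maximum length.
; StartInteract plays a timeline that lerps the cube's rotation.
; The beam refreshes only at BeginPlay and during that timeline, not every tick.
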(event `LaserUpdate`
  (bind _arrow (`self.Arrow`))
  (bind _returnvalue (`SceneComponent.K2_GetComponentLocation` _arrow))
  ; Cast Laser and Lenth
  (bind _outhit (`KismetSystemLibrary.LineTraceSingle` _returnvalue (+ _returnvalue (* (`SceneComponent.GetForwardVector` _arrow) (`self.LaserLength`))) "TraceTypeQuery1"))
  (bind (_bblockinghit _binitialoverlap _time _distance) (`GameplayStatics.BreakHitResult` _outhit))
  (if _bblockinghit
    (bind _output_get (set `self.MeshLength` _distance))
    (`SceneComponent.SetWorldScale3D` (`self.LaserCylinder`) (`KismetMathLibrary.MakeVector` (/ _output_get 10.0) 20.0 20.0))
    (else
      (bind _output_get_2 (set `self.MeshLength` (`self.LaserLength`)))
      (`SceneComponent.SetWorldScale3D` (`self.LaserCylinder`) (`KismetMathLibrary.MakeVector` (/ _output_get_2 10.0) 20.0 20.0)))))

(event `self.ReceiveBeginPlay`
  (`self.LaserUpdate`))

(event `/Game/Blueprints/LaserMiniGame/BPI_FreakInteract.StartInteract`
  ; Rotation Object after interact
  (`KismetSystemLibrary.PrintString` (`KismetSystemLibrary.GetDisplayName` self))
  (bind _output_get (set `self.InicialRotation` (`SceneComponent.RelativeRotation` (`self.Cube`))))
  (set `self.ResultRotation` (`KismetMathLibrary.MakeRotator` (.roll _output_get) (.pitch _output_get) (+ (.yaw _output_get) 45.0)))
  (bind (_direction _rotate) (`Timeline|Timeline` :!via `PlayFromStart`)
    (:`Update`
      (`self.LaserUpdate`)
      (`SceneComponent.K2_SetRelativeRotation` (`self.Cube`) (`KismetMathLibrary.RLerp` (`self.InicialRotation`) (`self.ResultRotation`) _rotate) false false))))

(fn `UserConstructionScript`)