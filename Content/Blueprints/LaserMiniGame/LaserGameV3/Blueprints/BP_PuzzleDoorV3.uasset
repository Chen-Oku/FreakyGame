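; BP_PuzzleDoorV3 is the laser puzzle's exit door, a clown whose mouth opens to reveal a portal that ends the level.
; An external activation plays the clown montage once with a camera shake, then after a short delay shows the portal, fading its opacity via a timeline with a Niagara vortex.
; The portal's trigger, disabled until then, loads the Credits level when the player overlaps it.
; Deactivation does nothing, and older sliding-door logic remains unconnected.
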(event `self.OnReceiverActivated`)

(event `self.ReceiveBeginPlay`
  (`SceneComponent.SetVisibility` (`self.Portal`) false false)
  (`PrimitiveComponent.SetCollisionEnabled` (`self.EndLevelTrigger`) "NoCollision"))

(event `self.BPC_External.ExternalActivate`
  (params (ApplyConditions :type Boolean))
  (if (not (`self.bIsOpen`))
    (`|PlayMontage` (`self.ClownActor`) "/Game/Mesh/Fish/Clown/AM_Clown.AM_Clown" 1.0 0.0 "OpenMouth"
      (:`then`
        (`GameplayStatics.PlayWorldCameraShake` "/Game/Blueprints/SharedCamera/CS_RumbleCamera.CS_RumbleCamera_C" (`self.K2_GetActorLocation`) 500.0 5000.0)
        (set `self.bIsOpen` true)
        (`KismetSystemLibrary.Delay` 1.0)
        (`SceneComponent.SetVisibility` (`self.Portal`) true false)
        (`PrimitiveComponent.SetCollisionEnabled` (`self.EndLevelTrigger`) "QueryOnly")
        (bind (_direction _fadeinportal) (`Timeline|Timeline`)
          (:`Update`
            (`MeshComponent.SetScalarParameterValueOnMaterials` (`self.Portal`) "Opacity" _fadeinportal)
            (`ActorComponent.Activate` (`self.NS_PortalVortex`) false)))))))

(event `self.EndLevelTrigger.OnComponentBeginOverlap`
  (params (OverlappedComponent :type "PrimitiveComponent Object Reference") (OtherActor :type "Actor Object Reference") (OtherComp :type "PrimitiveComponent Object Reference") (OtherBodyIndex :type Integer) (bFromSweep :type Boolean) (SweepResult :type "HitResult Structure (by ref)"))
  (cast `/Game/Blueprints/PlayerZD/BP_PlayerCharacterZD` OtherActor)
  (`GameplayStatics.OpenLevel` "Credits"))

(event `self.BPC_External.ExternalDeactivate`
  (params (ApplyConditions :type Boolean)))

(fn `CanReceiveLaser?`
  (returns (bCanReceive :type Boolean))
  (return false))

(fn `UserConstructionScript`)