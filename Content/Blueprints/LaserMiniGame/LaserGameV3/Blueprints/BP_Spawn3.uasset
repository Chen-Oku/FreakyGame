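; BP_Spawn3 is a laser spawn point for the laser mini-game that exposes TurnOnLaser and TurnOffLaser functions.
; It pairs an emitter (BPSEmitter1) with a handler (BPCHandler1), and starts with the emitter deactivated, printing a debug message on BeginPlay.
; Turning on only calls the handler's activation, while turning off deactivates the emitter directly and then the handler.
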(event `self.ReceiveBeginPlay`
  (`KismetSystemLibrary.PrintString` "APAGADO")
  (`/Game/Blueprints/LaserMiniGame/LaserGameV3/Blueprints/BuildingBlocks/BPS_Emitter.DeactivateLaser` (`self.BPS_Emitter1`)))

(fn `TurnOffLaser`
  (`/Game/Blueprints/LaserMiniGame/LaserGameV3/Blueprints/BuildingBlocks/BPS_Emitter.DeactivateLaser` (`self.BPS_Emitter1`))
  (`/Game/Blueprints/LaserMiniGame/LaserGameV3/Blueprints/BuildingBlocks/BPC_Handler.DeactivateHandler` (`self.BPC_Handler1`) null))

(fn `TurnOnLaser`
  (`/Game/Blueprints/LaserMiniGame/LaserGameV3/Blueprints/BuildingBlocks/BPC_Handler.ActivateHandler` (`self.BPC_Handler1`) null))

(fn `UserConstructionScript`)