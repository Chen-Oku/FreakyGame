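; BP_LaserReceiverV3 is a laser receiver for the V3 laser minigame, with most of its logic disconnected.
; LaserStop resets its timer and activated flag, while LaserUpdate and the handler component's activate and deactivate events are empty.
; Unconnected nodes hold a hold-time check, gated by an always-true CanReceiveLaser, that would activate it once and message a door.
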(event `self.LaserUpdate`
  (params (HitLocation :type "Vector Structure") (HitNormal :type "Vector Structure") (IncomingDirection :type "Vector Structure") (BouncesRemain :type Integer) (SourceActor :type "Actor Object Reference") (MirrorActor :type "Array of /Game/Blueprints/LaserMiniGame/MirrorMiniGame/BP_Mirror Object Reference (by ref)")))

(event `self.LaserStop`
  (params (SourceActor :type "Actor Object Reference"))
  (set `self.CurrentLaserTime` 0.0)
  (set `self.bIsActivated` false))

(event `self.BPC_Handler.ActivateHandler`
  (params (Instigator :type "/Game/Blueprints/LaserMiniGame/LaserGameV3/Blueprints/BuildingBlocks/BPC_Handler Object Reference")))

(event `self.BPC_Handler.DeactivateHandler`
  (params (Instigator :type "/Game/Blueprints/LaserMiniGame/LaserGameV3/Blueprints/BuildingBlocks/BPC_Handler Object Reference")))

(fn `CanReceiveLaser?`
  (returns (bCanReceive :type Boolean))
  (return true))

(fn `UserConstructionScript`)