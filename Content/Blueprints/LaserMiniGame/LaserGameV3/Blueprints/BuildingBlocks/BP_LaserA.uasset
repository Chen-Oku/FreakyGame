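; BP_LaserA is a colored laser beam segment actor for the laser minigame.
; Each tick it multi-traces forward, stretches the beam mesh, positions emitter and bounce effects, and passes hits to BPC_Handler components.
; Set differences between frames drive start, update and stop messages, while a recursive check of upstream lasers prevents loops.
; Color changes propagate to hit handlers, and LaserStopHitting notifies them before destroying the beam.
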(event `self.ReceiveBeginPlay`
  (bind _coloroverride (`self.ColorOverride`))
  (bind _returnvalue (* _coloroverride (struct :`R` 50.0 :`G` 50.0 :`B` 50.0 :`A` 1.0)))
  (bind _returnvalue_2 (`KismetMaterialLibrary.CreateDynamicMaterialInstance` "/Game/Materials/LaserMaterials/MI_LaserRay.MI_LaserRay"))
  (set `self.Material Instance` _returnvalue_2)
  (`PrimitiveComponent.SetMaterial` (`self.StaticMesh`) 0 (`self.Material Instance`))
  (bind _returnvalue_3 (`KismetMaterialLibrary.CreateDynamicMaterialInstance` "/Game/Materials/LaserMaterials/MI_Laser.MI_Laser"))
  (set `self.Material Instance1` _returnvalue_3)
  (`PrimitiveComponent.SetMaterial` (`self.StaticMesh`) 1 (`self.Material Instance1`))
  (`self.ChangeLaserColor` _coloroverride)
  (`FXSystemComponent.SetColorParameter` (`self.NS_LightBounce`) "LaserColorVFX" _returnvalue)
  (`FXSystemComponent.SetColorParameter` (`self.NS_LightEmitter`) "LaserColorVFX" _returnvalue))

(event `self.ReceiveTick`
  (params (DeltaSeconds :type "Float (single-precision)"))
  (bind (_star _end) (`self.CalculateLaserTrace`))
  (bind _ns_lightbounce (`self.NS_LightBounce`))
  (bind _ns_lightemitter (`self.NS_LightEmitter`))
  (`ActorComponent.Activate` _ns_lightemitter false)
  (`SceneComponent.K2_SetWorldLocation` _ns_lightemitter _star false false)
  (bind (_outhits _returnvalue) (`KismetSystemLibrary.LineTraceMulti` _star _end "TraceTypeQuery3" false (`self.ActorsToIgnore`)))
  (if _returnvalue
    (for _array_element _outhits
      (`|ExecutionSequence`
        (:`then_0`
          (bind (_bblockinghit _binitialoverlap _time _distance _location _impactpoint _normal _impactnormal _physmat _hitactor _hitcomponent _hitbonename _bonename _hititem _elementindex _faceindex _tracestart _traceend) (`GameplayStatics.BreakHitResult` _array_element))
          (if _bblockinghit
            (`self.UpdateLength` _distance)
            (`ActorComponent.Activate` _ns_lightbounce false)
            (`SceneComponent.K2_SetWorldLocation` _ns_lightbounce (`KismetMathLibrary.SelectVector` _impactpoint _traceend _bblockinghit) false false)))
        (:`then_1`
          (`self.HandleHitActors` _array_element))))
    (else
      (`self.UpdateLength` (`self.Range`))
      (`SceneComponent.K2_SetWorldLocation` (`self.NS_LightBounce`) (`.End` (`self.CalculateLaserTrace`)) false false)))
  (bind _result (`BlueprintSetLibrary.Set_Difference` (`self.PreviouslyHitHandler`) (`self.Current Hit Handler`)))
  (bind _result_2 (`BlueprintSetLibrary.Set_ToArray` _result))
  (for _array_element_2 _result_2
    (message `/Game/Blueprints/LaserMiniGame/LaserGameV3/Blueprints/BuildingBlocks/BPI_LasersA.LaserStopHitting` _array_element_2 self)
    (`BlueprintMapLibrary.Map_Remove` (`self.HittingHandler`) _array_element_2))
  (set `self.PreviouslyHitHandler` (`self.Current Hit Handler`))
  (`BlueprintSetLibrary.Set_Clear` (`self.Current Hit Handler`)))

(event `/Game/Blueprints/LaserMiniGame/LaserGameV3/Blueprints/BuildingBlocks/BPI_LasersA.LaserStopHitting`
  (params (Input :type "/Game/Blueprints/LaserMiniGame/LaserGameV3/Blueprints/BuildingBlocks/BP_LaserA Object Reference"))
  (`|ExecutionSequence`
    (:`then_0`
      (bind _result (`BlueprintSetLibrary.Set_ToArray` (`self.PreviouslyHitHandler`)))
      (for _array_element _result
        (message `/Game/Blueprints/LaserMiniGame/LaserGameV3/Blueprints/BuildingBlocks/BPI_LasersA.LaserStopHitting` _array_element self)))
    (:`then_1`
      (`self.K2_DestroyActor`))))

(fn `CalculateLaserTrace`
  (returns (Star :type "Vector Structure") (End :type "Vector Structure"))
  (bind _returnvalue (`self.K2_GetActorLocation`))
  (return _returnvalue (+ _returnvalue (* (`self.GetActorForwardVector`) (`self.Range`)))))

(fn `ChangeLaserColor`
  (params (Value :type "LinearColor Structure"))
  (set `self.ColorOverride` Value)
  (`MaterialInstanceDynamic.SetVectorParameterValue` (`self.Material Instance`) "Color" Value)
  (`MaterialInstanceDynamic.SetVectorParameterValue` (`self.Material Instance1`) "Color" Value)
  (bind _result (`BlueprintSetLibrary.Set_ToArray` (`self.PreviouslyHitHandler`)))
  (for _array_element _result
    (`/Game/Blueprints/LaserMiniGame/LaserGameV3/Blueprints/BuildingBlocks/BPC_Handler.IntermediateChange` _array_element self)))

(fn `GetHitByHandler`
  (params (Key :type "/Game/Blueprints/LaserMiniGame/LaserGameV3/Blueprints/BuildingBlocks/BPC_Handler Object Reference (by ref)"))
  (returns (Value :type "HitResult Structure") (ReturnValue :type Boolean))
  (bind (_value _returnvalue) (`BlueprintMapLibrary.Map_Find` (`self.HittingHandler`) Key))
  (return _value _returnvalue))

(fn `HandleHitActors`
  (params (InputPin :type "HitResult Structure"))
  (locals (`L-Handler` :type "/Game/Blueprints/LaserMiniGame/LaserGameV3/Blueprints/BuildingBlocks/BPC_Handler Object Reference"))
  (bind _returnvalue (`self.GetComponentByClass` (`.HitActor` (`GameplayStatics.BreakHitResult` InputPin)) "/Game/Blueprints/LaserMiniGame/LaserGameV3/Blueprints/BuildingBlocks/BPC_Handler.BPC_Handler_C"))
  (`/Engine/EditorBlueprintResources/StandardMacros.IsValid` _returnvalue
    (:`Is Valid`
      (set `local.L-Handler` _returnvalue)
      (if (`self.IsNotOnPath` (`local.L-Handler`))
        (`BlueprintMapLibrary.Map_Add` (`self.HittingHandler`) (`local.L-Handler`) (`local.InputPin`))
        (if (`BlueprintSetLibrary.Set_Contains` (`self.PreviouslyHitHandler`) (`local.L-Handler`))
          (`/Game/Blueprints/LaserMiniGame/LaserGameV3/Blueprints/BuildingBlocks/BPC_Handler.LaserUpdateHitting` (`local.L-Handler`) self (`local.InputPin`))
          (else
            (message `/Game/Blueprints/LaserMiniGame/LaserGameV3/Blueprints/BuildingBlocks/BPI_LasersA.LaserStartHitting` (`local.L-Handler`) self (`local.InputPin`))))
        (`BlueprintSetLibrary.Set_Add` (`self.Current Hit Handler`) (`local.L-Handler`))))))

(fn `IsNotOnPath`
  (params (InputHandler :type "/Game/Blueprints/LaserMiniGame/LaserGameV3/Blueprints/BuildingBlocks/BPC_Handler Object Reference"))
  (returns (OutputPin :type Boolean))
  (locals (`L-CurrentLaser` :type "/Game/Blueprints/LaserMiniGame/LaserGameV3/Blueprints/BuildingBlocks/BP_LaserA Object Reference"))
  (bind _l_currentlaser (`local.L-CurrentLaser`))
  (if (`KismetArrayLibrary.Array_IsNotEmpty` (`self.PreviousLasers`))
    (for _array_element (`self.PreviousLasers`)
      (bind _output_get (set `local.L-CurrentLaser` _array_element))
      (if (== (`/Game/Blueprints/LaserMiniGame/LaserGameV3/Blueprints/BuildingBlocks/BP_LaserA.OwningHandler` _output_get) (`local.InputHandler`))
        (return false)
        (else
          (`/Engine/EditorBlueprintResources/StandardMacros.IsValid` _l_currentlaser
            (:`Is Valid`
              (if (not (`self.IsNotOnPath` _l_currentlaser (`local.InputHandler`)))
                (return false)))
            (:`Is Not Valid`
              (return false))))))
    (return true)
    (else
      (return true))))

(fn `UpdateLength`
  (params (InputPin :type "Float (single-precision)"))
  (if (not (`KismetMathLibrary.NearlyEqual_FloatFloat` InputPin (`self.PreviousLength`) 2.0))
    (bind _output_get (set `self.PreviousLength` (`local.InputPin`)))
    (`SceneComponent.SetWorldScale3D` (`self.StaticMesh`) (`KismetMathLibrary.MakeVector` 1.5 1.5 (/ _output_get 100.0)))))

(fn `UserConstructionScript`)