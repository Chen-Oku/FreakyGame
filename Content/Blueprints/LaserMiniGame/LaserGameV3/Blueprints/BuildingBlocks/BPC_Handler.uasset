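; Laser puzzle component that decides when its owning actor activates or deactivates, based on lasers hitting it and linked external components.
; Tracks incoming lasers, filters excluded colors, and checks individual or merged colors against LaserRules.
; Relays hit, color and forced-activation changes to sibling components implementing BPI_LasersA, then calls its activate and deactivate handlers.
; An optional reversible looping timer delays switching and reports progress as an alpha.
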(event `self.ReceiveBeginPlay`
  (`|ExecutionSequence`
    (:`then_0`
      (bind _output_get (set `self.LinkedComponent` (`Actor.GetComponentsByInterface` (`self.GetOwner`) "/Game/Blueprints/LaserMiniGame/LaserGameV3/Blueprints/BuildingBlocks/BPI_LasersA.BPI_LasersA_C")))
      (`KismetArrayLibrary.Array_RemoveItem` _output_get self)
      (for _array_element (`Actor.K2_GetComponentsByClass` (`self.GetOwner`) "/Script/Engine.StaticMeshComponent")
        (`PrimitiveComponent.SetCollisionResponseToChannel` _array_element "ECC_GameTraceChannel1" (select `bool` (`self.IsBlocking`) :`false` "ECR_Overlap" :`true` "ECR_Block" :!type "ECollisionResponse Enum"))))
    (:`then_1`
      (if (`self.InvertSystem`)
        (for _array_element_2 (`Actor.K2_GetComponentsByClass` (`self.GetOwner`) "/Game/Blueprints/LaserMiniGame/LaserGameV3/Blueprints/BuildingBlocks/BPS_Emitter.BPS_Emitter_C")
          (`/Game/Blueprints/LaserMiniGame/LaserGameV3/Blueprints/BuildingBlocks/BPS_Emitter.SetLaserColor` _array_element_2)
          (`/Game/Blueprints/LaserMiniGame/LaserGameV3/Blueprints/BuildingBlocks/BPS_Emitter.LaserStopHitting` _array_element_2 null))))
    (:`then_2`
      (for (_array_element_3 _array_index) (`self.LaserRules`)
        (`KismetArrayLibrary.Array_Set` (`self.LaserRules`) _array_index (`self.SetAlphaTo1` _array_element_3)))
      (for (_array_element_4 _array_index_2) (`self.LaserFilter`)
        (`KismetArrayLibrary.Array_Set` (`self.LaserFilter`) _array_index_2 (`self.SetAlphaTo1` _array_element_4))))))

(event `CE_TimerFinishedActivate`
  (bind _array_element (`self.ForEachComponent` :!label _label)
    (:`LoopBody`
      (message `/Game/Blueprints/LaserMiniGame/LaserGameV3/Blueprints/BuildingBlocks/BPI_LasersA.LaserStartHitting` _array_element (stale `/Game/Blueprints/LaserMiniGame/LaserGameV3/Blueprints/BuildingBlocks/BPI_LasersA.LaserStartHitting` Input) (stale `/Game/Blueprints/LaserMiniGame/LaserGameV3/Blueprints/BuildingBlocks/BPI_LasersA.LaserStartHitting` `Hit Info`)))
    (:`Completed`
      (`self.ActivateHandler` self))))

(event `CE_ActivateOverride`
  (if (not (`self.UseTimer`)) :!label _label_2
    (goto _label)
    (else
      (set `self.ReverseTimer` false)
      (`self.StartTimer` false))))

(event `/Game/Blueprints/LaserMiniGame/LaserGameV3/Blueprints/BuildingBlocks/BPI_LasersA.LaserStartHitting`
  (params (Input :type "/Game/Blueprints/LaserMiniGame/LaserGameV3/Blueprints/BuildingBlocks/BP_LaserA Object Reference") (`Hit Info` :type "HitResult Structure"))
  (`self.LaserAdded` Input)
  (`self.IsNotLocked`
    (:`NotLocked`
      (if (`self.CanActivate`)
        (goto _label_2)))))

(event `CE_DeactivateOverride`
  (if (not (`self.UseTimer`)) :!label _label_3
    (bind _array_element (`self.ForEachComponent` :!label _label_4)
      (:`LoopBody`
        (message `/Game/Blueprints/LaserMiniGame/LaserGameV3/Blueprints/BuildingBlocks/BPI_LasersA.LaserStopHitting` _array_element (stale `/Game/Blueprints/LaserMiniGame/LaserGameV3/Blueprints/BuildingBlocks/BPI_LasersA.LaserStopHitting` Input)))
      (:`Completed`
        (`self.ComponentColorChange` (stale `/Game/Blueprints/LaserMiniGame/LaserGameV3/Blueprints/BuildingBlocks/BPI_LasersA.LaserStopHitting` Input))
        (`self.DeactivateHandler` self)))
    (else
      (set `self.ReverseTimer` true)
      (`self.StartTimer` false))))

(event `CE_TimerFinishedDeactivate`
  (goto _label_4))

(event `/Game/Blueprints/LaserMiniGame/LaserGameV3/Blueprints/BuildingBlocks/BPI_LasersA.LaserStopHitting`
  (params (Input :type "/Game/Blueprints/LaserMiniGame/LaserGameV3/Blueprints/BuildingBlocks/BP_LaserA Object Reference"))
  (`self.LaserRemoved` Input)
  (`self.IsNotLocked`
    (:`NotLocked`
      (if (not (`self.CanActivate`))
        (goto _label_3)
        (else
          (`self.ComponentColorChange` Input))))))

(event `/Game/Blueprints/LaserMiniGame/LaserGameV3/Blueprints/BuildingBlocks/BPI_LasersA.LaserUpdateHitting`
  (params (Input :type "/Game/Blueprints/LaserMiniGame/LaserGameV3/Blueprints/BuildingBlocks/BP_LaserA Object Reference") (`Hit Info` :type "HitResult Structure"))
  (bind _array_element (`self.ForEachComponent`)
    (:`LoopBody`
      (message `/Game/Blueprints/LaserMiniGame/LaserGameV3/Blueprints/BuildingBlocks/BPI_LasersA.LaserUpdateHitting` _array_element Input `Hit Info`))))

(event `/Game/Blueprints/LaserMiniGame/LaserGameV3/Blueprints/BuildingBlocks/BPI_LasersA.IntermediateChange`
  (params (Modified :type "/Game/Blueprints/LaserMiniGame/LaserGameV3/Blueprints/BuildingBlocks/BP_LaserA Object Reference"))
  (`self.RecalculateColor` Modified))

(event `CE_Ext_TimerActivate`
  (bind _array_element (`self.ForEachComponent` :!label _label_5)
    (:`LoopBody`
      (message `/Game/Blueprints/LaserMiniGame/LaserGameV3/Blueprints/BuildingBlocks/BPI_LasersA.ForceActivation` _array_element (stale `/Game/Blueprints/LaserMiniGame/LaserGameV3/Blueprints/BuildingBlocks/BPI_LasersA.ForceActivation` ApplyConditions)))
    (:`Completed`
      (`self.ActivateHandler` self))))

(event `/Game/Blueprints/LaserMiniGame/LaserGameV3/Blueprints/BuildingBlocks/BPI_LasersA.ForceActivation`
  (params (ApplyConditions :type Boolean))
  (if ApplyConditions
    (if (`self.CanActivate`)
      (if (`self.AreAllCompsActivated`) :!label _label_6
        (if (not (`self.UseTimer`))
          (goto _label_5)
          (else
            (set `self.ReverseTimer` false)
            (`self.StartTimer` true)))))
    (else
      (goto _label_6))))

(event `CE_Ext_TimerDeactivate`
  (bind _array_element (`self.ForEachComponent` :!label _label_7)
    (:`LoopBody`
      (message `/Game/Blueprints/LaserMiniGame/LaserGameV3/Blueprints/BuildingBlocks/BPI_LasersA.ForceDeactivation` _array_element (stale `/Game/Blueprints/LaserMiniGame/LaserGameV3/Blueprints/BuildingBlocks/BPI_LasersA.ForceDeactivation` ApplyConditions)))
    (:`Completed`
      (`self.ComponentColorChange` null)
      (`self.DeactivateHandler` self))))

(event `/Game/Blueprints/LaserMiniGame/LaserGameV3/Blueprints/BuildingBlocks/BPI_LasersA.ForceDeactivation`
  (params (ApplyConditions :type Boolean))
  (if ApplyConditions
    (if (not (`self.CanActivate`))
      (if (not (`self.UseTimer`)) :!label _label_8
        (goto _label_7)
        (else
          (set `self.ReverseTimer` true)
          (`self.StartTimer` true))))
    (else
      (goto _label_8))))

(fn `AreAllCompsActivated`
  (returns (ReturnValue :type Boolean))
  (for _array_element (`self.LinkedExternalComps`)
    (if (not (`/Game/Blueprints/LaserMiniGame/LaserGameV3/Blueprints/BuildingBlocks/BPC_External.IsCompActivated` _array_element))
      (return false)))
  (return true))

(fn `CanActivate`
  (returns (`Output Pin` :type Boolean))
  (locals (L_FilteredLasers :type "Array of /Game/Blueprints/LaserMiniGame/LaserGameV3/Blueprints/BuildingBlocks/BP_LaserA Object Reference") (L_Counter :type Integer) (L_CurrentColor :type "LinearColor Structure"))
  (bind _output_get (set `local.L_FilteredLasers` (`self.FilteredLasers`)))
  (if (and (`KismetArrayLibrary.Array_IsEmpty` _output_get) (not (`self.IsLinked`)))
    (return false)
    (elif (`KismetArrayLibrary.Array_IsEmpty` (`self.LaserRules`))
      (if (`self.IsLinked`)
        (return (`self.AreAllCompsActivated`))
        (else
          (return true)))
      (elif (> (`KismetArrayLibrary.Array_Length` (`self.LaserRules`)) (`KismetArrayLibrary.Array_Length` (`local.L_FilteredLasers`)))
        (return false)
        (elif (`self.CanMergeColor`)
          (for _array_element (`self.LaserRules`)
            (if (or (`self.ColorEqual` (struct) _array_element) (`self.DoesContainColor` (`self.GetMergeColor`) _array_element))
              (`/Engine/EditorBlueprintResources/StandardMacros.IncrementInt` (`local.L_Counter`))))
          (return (and (== (`KismetArrayLibrary.Array_Length` (`self.LaserRules`)) (`local.L_Counter`)) (or (not (`self.IsLinked`)) (`self.AllLinksActivated`))))
          (else
            (for _array_element_2 (`self.LaserRules`)
              (bind _output_get_2 (set `local.L_CurrentColor` _array_element_2))
              (if (not (`self.ColorEqual` _output_get_2))
                (for (_array_element_3 _array_index) (`local.L_FilteredLasers`)
                  (if (`self.DoesContainColor` (`/Game/Blueprints/LaserMiniGame/LaserGameV3/Blueprints/BuildingBlocks/BP_LaserA.ColorOverride` _array_element_3) (`local.L_CurrentColor`))
                    (`/Engine/EditorBlueprintResources/StandardMacros.IncrementInt` (`local.L_Counter`)
                      (:`  `
                        (`KismetArrayLibrary.Array_Remove` (`local.L_FilteredLasers`) _array_index)
                        (break)))))
                (else
                  (`/Engine/EditorBlueprintResources/StandardMacros.IncrementInt` (`local.L_Counter`)))))
            (return (and (== (`KismetArrayLibrary.Array_Length` (`self.LaserRules`)) (`local.L_Counter`)) (or (not (`self.IsLinked`)) (`self.AllLinksActivated`))))))))))

(fn `ComponentColorChange`
  (params (Modified :type "/Game/Blueprints/LaserMiniGame/LaserGameV3/Blueprints/BuildingBlocks/BP_LaserA Object Reference"))
  (bind _array_element (`self.ForEachComponent`)
    (:`LoopBody`
      (message `/Game/Blueprints/LaserMiniGame/LaserGameV3/Blueprints/BuildingBlocks/BPI_LasersA.IntermediateChange` _array_element Modified))))

(fn `DoesContainColor`
  (params (Input :type "LinearColor Structure") (Condition :type "LinearColor Structure"))
  (returns (ReturnValue :type Boolean))
  (bind ((`R` _r) (`G` _g) (`B` _b)) (break `LinearColor` (`local.Condition`)))
  (bind ((`R` _r_2) (`G` _g_2) (`B` _b_2)) (break `LinearColor` (`local.Input`)))
  (if (`self.UseColorValue`)
    (return (and (>= _r_2 _r) (>= _g_2 _g) (>= _b_2 _b)))
    (else
      (return (`self.ColorEqual` (`local.Input`) (`local.Condition`))))))

(fn `ExternalUpdateTimer`
  (if (select `bool` (`self.ReverseTimer`) :`false` (>= (`self.TimerAlpha`) 1.0) :`true` (<= (`self.TimerAlpha`) 0.0))
    (`KismetSystemLibrary.K2_ClearAndInvalidateTimerHandle` (`self.TimerHandle`))
    (if (`self.ReverseTimer`)
      (`self.CE_Ext_TimerDeactivate`)
      (else
        (`self.CE_Ext_TimerActivate`)))
    (else
      (set `self.TimerAlpha` (+ (* (* (/ 1.0 (`self.Duration`)) (`self.Substep`)) (`KismetMathLibrary.SelectFloat` -1.0 1.0 (`self.ReverseTimer`))) (`self.TimerAlpha`)))
      (`self.UpdateHandler` (`self.TimerAlpha`)))))

(fn `GetMergeColor`
  (returns (ReturnValue :type "LinearColor Structure"))
  (bind (_r _g _b) (`KismetMathLibrary.BreakColor` (`self.MergeColor`)))
  (return (`KismetMathLibrary.MakeColor` (`KismetMathLibrary.FClamp` _r) (`KismetMathLibrary.FClamp` _g) (`KismetMathLibrary.FClamp` _b))))

(fn `GetVisibleColor`
  (returns (PassByColor :type "LinearColor Structure"))
  (bind _lasersinqueue (`self.LasersInQueue`))
  (bind _output (`|GetArrayItem` (`self.LasersInQueue`)))
  (bind _output_2 (`|GetArrayItem` _lasersinqueue (`KismetArrayLibrary.Array_LastIndex` _lasersinqueue)))
  (`|ExecutionSequence`
    (:`then_0`
      (switch `/Game/Blueprints/LaserMiniGame/LaserGameV3/Blueprints/BuildingBlocks/E_ColorSelection` (`self.UsedColors`)
        (:`NewEnumerator0`
          (`/Engine/EditorBlueprintResources/StandardMacros.IsValid` _output
            (:`Is Valid`
              (bind _output_get (set `self.PassByColor` (`/Game/Blueprints/LaserMiniGame/LaserGameV3/Blueprints/BuildingBlocks/BP_LaserA.ColorOverride` _output)))
              (return _output_get))
            (:`Is Not Valid`
              (return (`self.PassByColor`)))))
        (:`NewEnumerator1`
          (`/Engine/EditorBlueprintResources/StandardMacros.IsValid` _output_2
            (:`Is Valid`
              (set `self.PassByColor` (`/Game/Blueprints/LaserMiniGame/LaserGameV3/Blueprints/BuildingBlocks/BP_LaserA.ColorOverride` _output_2))
              (return (`self.PassByColor`)))))
        (:`NewEnumerator2`
          (set `self.PassByColor` (`self.GetMergeColor`))
          (return (`self.PassByColor`)))))
    (:`then_1`
      (return (`self.PassByColor`)))))

(fn `IsLaserFiltered`
  (params (`Laser In` :type "/Game/Blueprints/LaserMiniGame/LaserGameV3/Blueprints/BuildingBlocks/BP_LaserA Object Reference"))
  (returns (ReturnValue :type Boolean))
  (return (`KismetArrayLibrary.Array_Contains` (`self.LaserFilter`) (`self.SetAlphaTo1` (`/Game/Blueprints/LaserMiniGame/LaserGameV3/Blueprints/BuildingBlocks/BP_LaserA.ColorOverride` (`local.Laser In`))))))

(fn `LaserAdded`
  (params (NewItem :type "/Game/Blueprints/LaserMiniGame/LaserGameV3/Blueprints/BuildingBlocks/BP_LaserA Object Reference (by ref)"))
  (`KismetArrayLibrary.Array_AddUnique` (`self.LasersInQueue`) NewItem)
  (if (not (`self.IsLaserFiltered` (`local.NewItem`)))
    (`KismetArrayLibrary.Array_AddUnique` (`self.FilteredLasers`) (`local.NewItem`))
    (if (or (`|EnumEquality` (`self.UsedColors`) "NewEnumerator0") (`self.CanMergeColor`))
      (set `self.MergeColor` (+ (`self.MergeColor`) (`/Game/Blueprints/LaserMiniGame/LaserGameV3/Blueprints/BuildingBlocks/BP_LaserA.ColorOverride` (`local.NewItem`)))))))

(fn `LaserRemoved`
  (params (NewItem :type "/Game/Blueprints/LaserMiniGame/LaserGameV3/Blueprints/BuildingBlocks/BP_LaserA Object Reference (by ref)"))
  (`KismetArrayLibrary.Array_RemoveItem` (`self.LasersInQueue`) NewItem)
  (if (not (`self.IsLaserFiltered` (`local.NewItem`)))
    (`KismetArrayLibrary.Array_RemoveItem` (`self.FilteredLasers`) (`local.NewItem`))
    (if (or (`|EnumEquality` (`self.UsedColors`) "NewEnumerator0") (`self.CanMergeColor`))
      (set `self.MergeColor` (- (`self.MergeColor`) (`/Game/Blueprints/LaserMiniGame/LaserGameV3/Blueprints/BuildingBlocks/BP_LaserA.ColorOverride` (`local.NewItem`)))))))

(fn `RecalculateColor`
  (params (InputPin :type "/Game/Blueprints/LaserMiniGame/LaserGameV3/Blueprints/BuildingBlocks/BP_LaserA Object Reference"))
  (`|ExecutionSequence`
    (:`then_0`
      (if (`|EnumEquality` (`self.UsedColors`) "NewEnumerator2")
        (set `self.MergeColor` (struct))
        (for _array_element (`self.LasersInQueue`)
          (set `self.MergeColor` (+ (`/Game/Blueprints/LaserMiniGame/LaserGameV3/Blueprints/BuildingBlocks/BP_LaserA.ColorOverride` _array_element) (`self.MergeColor`))))))
    (:`then_1`
      (`self.ComponentColorChange` (`local.InputPin`))
      (if (`self.CanActivate`)
        (`self.CE_ActivateOverride`)
        (else
          (`self.CE_DeactivateOverride`))))))

(fn `StartTimer`
  (params (ExternalTimer :type Boolean))
  (if (`KismetSystemLibrary.K2_TimerExistsHandle` (`self.TimerHandle`))
    (`KismetSystemLibrary.K2_ClearAndInvalidateTimerHandle` (`self.TimerHandle`)))
  (if (`local.ExternalTimer`)
    (bind _returnvalue (`KismetSystemLibrary.K2_SetTimerDelegate` (`|CreateDelegate` :!event `UpdateTimer`) (`self.Substep`) true))
    (set `self.TimerHandle` _returnvalue)
    (else
      (bind _returnvalue_2 (`KismetSystemLibrary.K2_SetTimerDelegate` (`|CreateDelegate` :!event `UpdateTimer`) (`self.Substep`) true))
      (set `self.TimerHandle` _returnvalue_2))))

(fn `UpdateTimer`
  (if (select `bool` (`self.ReverseTimer`) :`false` (>= (`self.TimerAlpha`) 1.0) :`true` (<= (`self.TimerAlpha`) 0.0))
    (`KismetSystemLibrary.K2_ClearAndInvalidateTimerHandle` (`self.TimerHandle`))
    (if (`self.ReverseTimer`)
      (`self.CE_TimerFinishedDeactivate`)
      (else
        (`self.CE_TimerFinishedActivate`)))
    (else
      (set `self.TimerAlpha` (+ (* (* (/ 1.0 (`self.Duration`)) (`self.Substep`)) (`KismetMathLibrary.SelectFloat` -1.0 1.0 (`self.ReverseTimer`))) (`self.TimerAlpha`)))
      (`self.UpdateHandler` (`self.TimerAlpha`)))))