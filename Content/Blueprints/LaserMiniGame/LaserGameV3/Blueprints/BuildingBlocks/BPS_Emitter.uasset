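; Laser mini-game emitter scene component that spawns and removes an outgoing laser (BP_LaserA) at its transform.
; It relies on the owner's BPC_Handler for incoming lasers, activation conditions and color merging.
; Hit and change events re-evaluate color, either overridden or taken from the handler, then toggle the attached laser.
; Inverted systems flip hit start/stop behavior, and forced activation can bypass spawn checks.
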(event `self.ReceiveBeginPlay`
  (bind _returnvalue (`Actor.GetComponentByClass` (`self.GetOwner`) "/Game/Blueprints/LaserMiniGame/LaserGameV3/Blueprints/BuildingBlocks/BPC_Handler.BPC_Handler_C"))
  (`/Engine/EditorBlueprintResources/StandardMacros.IsValid` _returnvalue
    (:`Is Valid`
      (set `self.OwningHandler` _returnvalue))))

(event `/Game/Blueprints/LaserMiniGame/LaserGameV3/Blueprints/BuildingBlocks/BPI_LasersA.LaserStartHitting`
  (params (Input :type "/Game/Blueprints/LaserMiniGame/LaserGameV3/Blueprints/BuildingBlocks/BP_LaserA Object Reference") (`Hit Info` :type "HitResult Structure"))
  (if (`self.isSystemInverted`)
    (`self.DeactivateLaser`)
    (else
      (`self.SetLaserColor` :!label _label)
      (if (`self.CanSpawnLaser`)
        (`self.AttachedLasers` :!label _label_2
          (:`then`)
          (:`else`
            (`self.ActivateLaser`)))))))

(event `/Game/Blueprints/LaserMiniGame/LaserGameV3/Blueprints/BuildingBlocks/BPI_LasersA.ForceActivation`
  (params (ApplyConditions :type Boolean))
  (if ApplyConditions
    (goto _label)
    (else
      (`self.SetLaserColor`)
      (goto _label_2))))

(event `/Game/Blueprints/LaserMiniGame/LaserGameV3/Blueprints/BuildingBlocks/BPI_LasersA.LaserStopHitting`
  (params (Input :type "/Game/Blueprints/LaserMiniGame/LaserGameV3/Blueprints/BuildingBlocks/BP_LaserA Object Reference"))
  (if (`self.isSystemInverted`)
    (`self.ActivateLaser`)
    (elif (not (`self.CanSpawnLaser`))
      (`self.DeactivateLaser` :!label _label_3))))

(event `/Game/Blueprints/LaserMiniGame/LaserGameV3/Blueprints/BuildingBlocks/BPI_LasersA.ForceDeactivation`
  (params (ApplyConditions :type Boolean))
  (goto _label_3))

(event `/Game/Blueprints/LaserMiniGame/LaserGameV3/Blueprints/BuildingBlocks/BPI_LasersA.IntermediateChange`
  (params (Modified :type "/Game/Blueprints/LaserMiniGame/LaserGameV3/Blueprints/BuildingBlocks/BP_LaserA Object Reference"))
  (if (not (`self.isSystemInverted`))
    (`self.SetLaserColor`)
    (if (`self.CanSpawnLaser`)
      (`self.AttachedLasers`
        (:`then`)
        (:`else`
          (`self.ActivateLaser`)))
      (else
        (`self.DeactivateLaser`)))))

(fn `ActivateLaser`
  (bind _returnvalue (`|SpawnActorFromClass` "/Game/Blueprints/LaserMiniGame/LaserGameV3/Blueprints/BuildingBlocks/BP_LaserA.BP_LaserA_C" (`self.K2_GetComponentToWorld`) "Undefined" "MultiplyWithRoot" null (`self.CurrentColor`) (`self.MaxRange`) (`self.GetFilteredLasers`) (`self.OwningHandler`) (`|MakeArray` (`self.GetOwner`)) null))
  (bind _output_get (set `self.AttachedLasers` _returnvalue))
  (`Actor.K2_AttachToComponent` _output_get self "None" "KeepWorld" "KeepWorld" "KeepWorld" false))

(fn `CanSpawnLaser`
  (returns (OutputPin :type Boolean))
  (if (`/Game/Blueprints/LaserMiniGame/LaserGameV3/Blueprints/BuildingBlocks/BPC_Handler.IsAdjustingColor` (`self.OwningHandler`))
    (if (`/Game/Blueprints/LaserMiniGame/LaserGameV3/Blueprints/BuildingBlocks/BPC_Handler.CanMergeColor` (`self.OwningHandler`))
      (return (`/Game/Blueprints/LaserMiniGame/LaserGameV3/Blueprints/BuildingBlocks/BPC_Handler.DoesContainColor` (`self.OwningHandler`) (`/Game/Blueprints/LaserMiniGame/LaserGameV3/Blueprints/BuildingBlocks/BPC_Handler.GetMergeColor` (`self.OwningHandler`)) (`self.OverrideColor`)))
      (else
        (for _array_element (`self.GetFilteredLasers`)
          (if (`/Game/Blueprints/LaserMiniGame/LaserGameV3/Blueprints/BuildingBlocks/BPC_Handler.DoesContainColor` (`self.OwningHandler`) (`/Game/Blueprints/LaserMiniGame/LaserGameV3/Blueprints/BuildingBlocks/BP_LaserA.ColorOverride` _array_element) (`self.OverrideColor`))
            (return true)))
        (return false)))
    (else
      (return (`/Game/Blueprints/LaserMiniGame/LaserGameV3/Blueprints/BuildingBlocks/BPC_Handler.CanActivate` (`self.OwningHandler`))))))

(fn `DeactivateLaser`
  (bind _attachedlasers (`self.AttachedLasers`)
    (:`then`
      (`/Game/Blueprints/LaserMiniGame/LaserGameV3/Blueprints/BuildingBlocks/BP_LaserA.LaserStopHitting` _attachedlasers null))
    (:`else`)))

(fn `DestroySelf`
  (`self.K2_DestroyComponent`))

(fn `SetLaserColor`
  (locals (`L-TempColor` :type "LinearColor Structure"))
  (`|ExecutionSequence`
    (:`then_0`
      (if (`self.UsedOverride`)
        (set `local.L-TempColor` (`self.OverrideColor`))
        (elif (`KismetArrayLibrary.Array_IsEmpty` (`/Game/Blueprints/LaserMiniGame/LaserGameV3/Blueprints/BuildingBlocks/BPC_Handler.FilteredLasers` (`self.OwningHandler`)))
          (set `local.L-TempColor` (`self.CurrentColor`))
          (else
            (set `local.L-TempColor` (`/Game/Blueprints/LaserMiniGame/LaserGameV3/Blueprints/BuildingBlocks/BPC_Handler.GetVisibleColor` (`self.OwningHandler`)))))))
    (:`then_1`
      (if (!= (`self.CurrentColor`) (`local.L-TempColor`))
        (set `self.CurrentColor` (`local.L-TempColor`))
        (bind _attachedlasers (`self.AttachedLasers`)
          (:`then`
            (`/Game/Blueprints/LaserMiniGame/LaserGameV3/Blueprints/BuildingBlocks/BP_LaserA.ChangeLaserColor` _attachedlasers (`self.CurrentColor`)))
          (:`else`))))))