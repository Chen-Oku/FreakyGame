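; BPC_Bounce is a laser minigame component that makes its owning actor bounce incoming lasers like a mirror.
; Each new hit spawns and activates a BPS_Emitter on the owner, mapped to its input laser, optionally copying that laser's color.
; Hit updates reposition the emitter through MirrorLocationRotation, and a hit ending stops and destroys it.
; IntermediateChange refreshes all bounced laser colors, and BeginPlay caches the owner's BPC_Handler.
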(event `self.ReceiveBeginPlay`
  (bind _returnvalue (`Actor.GetComponentByClass` (`self.GetOwner`) "/Game/Blueprints/LaserMiniGame/LaserGameV3/Blueprints/BuildingBlocks/BPC_Handler.BPC_Handler_C"))
  (`/Engine/EditorBlueprintResources/StandardMacros.IsValid` _returnvalue
    (:`Is Valid`
      (set `self.OwningHandler` _returnvalue))))

(event `/Game/Blueprints/LaserMiniGame/LaserGameV3/Blueprints/BuildingBlocks/BPI_LasersA.LaserStartHitting`
  (params (Input :type "/Game/Blueprints/LaserMiniGame/LaserGameV3/Blueprints/BuildingBlocks/BP_LaserA Object Reference") (`Hit Info` :type "HitResult Structure"))
  (`/Engine/EditorBlueprintResources/StandardMacros.IsValid` Input
    (:`Is Valid`
      (if (not (`BlueprintMapLibrary.Map_Contains` (`self.EmitterBounceMap`) Input))
        (`self.SpawnLaser` Input `Hit Info`)))))

(event `/Game/Blueprints/LaserMiniGame/LaserGameV3/Blueprints/BuildingBlocks/BPI_LasersA.LaserStopHitting`
  (params (Input :type "/Game/Blueprints/LaserMiniGame/LaserGameV3/Blueprints/BuildingBlocks/BP_LaserA Object Reference"))
  (`self.RemoveLaser` Input))

(event `/Game/Blueprints/LaserMiniGame/LaserGameV3/Blueprints/BuildingBlocks/BPI_LasersA.LaserUpdateHitting`
  (params (Input :type "/Game/Blueprints/LaserMiniGame/LaserGameV3/Blueprints/BuildingBlocks/BP_LaserA Object Reference") (`Hit Info` :type "HitResult Structure"))
  (bind (_location _rotation) (`self.MirrorLocationRotation` `Hit Info`))
  (bind (_value _returnvalue) (`BlueprintMapLibrary.Map_Find` (`self.EmitterBounceMap`) Input))
  (if _returnvalue
    (`SceneComponent.K2_SetWorldLocationAndRotation` _value _location _rotation false false)))

(event `/Game/Blueprints/LaserMiniGame/LaserGameV3/Blueprints/BuildingBlocks/BPI_LasersA.IntermediateChange`
  (params (Modified :type "/Game/Blueprints/LaserMiniGame/LaserGameV3/Blueprints/BuildingBlocks/BP_LaserA Object Reference"))
  (bind _values (`BlueprintMapLibrary.Map_Values` (`self.EmitterBounceMap`)))
  (for _array_element _values
    (`/Game/Blueprints/LaserMiniGame/LaserGameV3/Blueprints/BuildingBlocks/BPS_Emitter.SetLaserColor` _array_element)))

(fn `RemoveLaser`
  (params (InputPin :type "/Game/Blueprints/LaserMiniGame/LaserGameV3/Blueprints/BuildingBlocks/BP_LaserA Object Reference"))
  (locals (`L-RemoveItem` :type "/Game/Blueprints/LaserMiniGame/LaserGameV3/Blueprints/BuildingBlocks/BPS_Emitter Object Reference"))
  (bind (_value _returnvalue) (`BlueprintMapLibrary.Map_Find` (`self.EmitterBounceMap`) (`local.InputPin`)))
  (if _returnvalue
    (bind _output_get (set `local.L-RemoveItem` _value))
    (`/Game/Blueprints/LaserMiniGame/LaserGameV3/Blueprints/BuildingBlocks/BPS_Emitter.LaserStopHitting` _output_get null)
    (`/Game/Blueprints/LaserMiniGame/LaserGameV3/Blueprints/BuildingBlocks/BPS_Emitter.DestroySelf` (`local.L-RemoveItem`))
    (`BlueprintMapLibrary.Map_Remove` (`self.EmitterBounceMap`) (`local.InputPin`))))

(fn `SpawnLaser`
  (params (`Laser In` :type "/Game/Blueprints/LaserMiniGame/LaserGameV3/Blueprints/BuildingBlocks/BP_LaserA Object Reference") (`Hit Info` :type "HitResult Structure"))
  (bind _returnvalue (`Actor.GetTransform` (`self.GetOwner`)))
  (bind (_location _rotation) (`self.MirrorLocationRotation` (`local.Hit Info`)))
  (bind _returnvalue_2 (`|AddComponentByClass` (`self.GetOwner`) "/Game/Blueprints/LaserMiniGame/LaserGameV3/Blueprints/BuildingBlocks/BPS_Emitter.BPS_Emitter_C" false (`KismetMathLibrary.MakeTransform` (`KismetMathLibrary.InverseTransformLocation` _returnvalue _location) (`KismetMathLibrary.InverseTransformRotation` _returnvalue _rotation))))
  (`BlueprintMapLibrary.Map_Add` (`self.EmitterBounceMap`) (`local.Laser In`) _returnvalue_2)
  (if (`self.UseBounceColor`)
    (set `/Game/Blueprints/LaserMiniGame/LaserGameV3/Blueprints/BuildingBlocks/BPS_Emitter.OverrideColor` (`/Game/Blueprints/LaserMiniGame/LaserGameV3/Blueprints/BuildingBlocks/BP_LaserA.ColorOverride` (`local.Laser In`)) _returnvalue_2)
    (set `/Game/Blueprints/LaserMiniGame/LaserGameV3/Blueprints/BuildingBlocks/BPS_Emitter.UsedOverride` false _returnvalue_2))
  (`/Game/Blueprints/LaserMiniGame/LaserGameV3/Blueprints/BuildingBlocks/BPS_Emitter.SetLaserColor` _returnvalue_2)
  (`/Game/Blueprints/LaserMiniGame/LaserGameV3/Blueprints/BuildingBlocks/BPS_Emitter.ActivateLaser` _returnvalue_2))