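; BP_LaserTarget is the target object in the laser minigame, changing color according to whether a laser is hitting it.
; LaserBounce stores the hit response as the Active state and passes the hitting laser's color to PuzzleSolve.
; PuzzleSolve creates a dynamic M_Laser material on the inherited mesh and sets its base color to the laser color when active, or dark gray when not.
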(fn `LaserBounce`
  (params (P_LaserHit :type "/Game/Blueprints/LaserMiniGame/LaserGameV3/Blueprints/BP_LaserChild Object Reference") (P_HitResponce :type Boolean) (P_HitInfo :type "HitResult Structure"))
  (returns (NewLaser :type "/Game/Blueprints/LaserMiniGame/LaserGameV3/Blueprints/BP_LaserChild Object Reference"))
  (set `self.Active` P_HitResponce)
  (`self.Puzzle Solve` (`/Game/Blueprints/LaserMiniGame/LaserGameV3/Blueprints/BP_LaserParent.LaserColor` P_LaserHit))
  (return null))

(fn `Puzzle Solve`
  (params (`Color Laser` :type "LinearColor Structure"))
  (locals (NewLocalVar :type "StaticMeshComponent Object Reference"))
  (bind _returnvalue (`PrimitiveComponent.CreateDynamicMaterialInstance` (`self.SM_Parent`) 0 "/Game/Blueprints/LaserMiniGame/LaserGameV3/Materials/M_Laser.M_Laser" "None"))
  (`MaterialInstanceDynamic.SetVectorParameterValue` _returnvalue "Base Color" (`KismetMathLibrary.SelectColor` `Color Laser` (struct :`R` 0.270833 :`G` 0.270833 :`B` 0.270833 :`A` 1.0) (`self.Active`))))

(fn `UserConstructionScript`
  (`parent.UserConstructionScript`))