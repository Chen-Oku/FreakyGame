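; BP_Button is a pressure-style button for the laser minigame, triggered by overlaps on its Box.
; Each overlap raises the active count on the BPCExternal component, calling its ActivateThis when the count equals the required number.
; Activation sets IsLaserActivated, latching the button so later overlaps are ignored.
; Before that, ending an overlap lowers the clamped count and calls DeactivateThis.
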(event `self.Box.OnComponentBeginOverlap`
  (params (OverlappedComponent :type "PrimitiveComponent Object Reference") (OtherActor :type "Actor Object Reference") (OtherComp :type "PrimitiveComponent Object Reference") (OtherBodyIndex :type Integer) (bFromSweep :type Boolean) (SweepResult :type "HitResult Structure (by ref)"))
  (bind _bpc_external (`self.BPC_External`))
  ; Boton
  (if (not (`self.IsLaserActivated`))
    (bind _output_get (set `/Game/Blueprints/LaserMiniGame/LaserGameV3/Blueprints/BuildingBlocks/BPC_External.ActiveOverlaps` (+ (`/Game/Blueprints/LaserMiniGame/LaserGameV3/Blueprints/BuildingBlocks/BPC_External.ActiveOverlaps` _bpc_external) 1) _bpc_external))
    (if (== _output_get (`/Game/Blueprints/LaserMiniGame/LaserGameV3/Blueprints/BuildingBlocks/BPC_External.NecesaryCount` (`self.BPC_External`)))
      (`/Game/Blueprints/LaserMiniGame/LaserGameV3/Blueprints/BuildingBlocks/BPC_External.ActivateThis` (`self.BPC_External`) null)
      (set `self.IsLaserActivated` true))))

(event `self.Box.OnComponentEndOverlap`
  (params (OverlappedComponent :type "PrimitiveComponent Object Reference") (OtherActor :type "Actor Object Reference") (OtherComp :type "PrimitiveComponent Object Reference") (OtherBodyIndex :type Integer))
  (bind _bpc_external (`self.BPC_External`))
  ; Boton
  (if (not (`self.IsLaserActivated`))
    (set `/Game/Blueprints/LaserMiniGame/LaserGameV3/Blueprints/BuildingBlocks/BPC_External.ActiveOverlaps` (`KismetMathLibrary.Clamp` (- (`/Game/Blueprints/LaserMiniGame/LaserGameV3/Blueprints/BuildingBlocks/BPC_External.ActiveOverlaps` _bpc_external) 1) 0 2) _bpc_external)
    (`/Game/Blueprints/LaserMiniGame/LaserGameV3/Blueprints/BuildingBlocks/BPC_External.DeactivateThis` _bpc_external null)))

(fn `UserConstructionScript`)