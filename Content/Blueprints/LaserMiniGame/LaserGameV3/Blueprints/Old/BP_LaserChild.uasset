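; BP_LaserChild is a laser beam segment in the laser minigame, tinted through a dynamic material.
; Each tick it box-traces along its up vector and scales the beam mesh to the hit distance or maximum range.
; Hit changes notify actors through BPI_Laser and track the returned bounce laser, repositioned and rotated while a BP_ReflectLaser stays hit.
; CancelTargetHit notifies or deactivates the last target, then destroys the segment unless overridden.
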(event `self.ReceiveBeginPlay`
  (`self.ChangeColor`))

(event `self.ReceiveTick`
  (params (DeltaSeconds :type "Float (single-precision)"))
  (`self.Set End Point`))

(fn `Cancel Target Hit`
  (params (Override :type Boolean))
  (returns (`Remove From Array` :type Boolean))
  (`|ExecutionSequence`
    (:`then_0`
      (bind _lasthitactor (`self.LastHitActor`)
        (:`then`
          (bind _asbp_laser_parent (cast `/Game/Blueprints/LaserMiniGame/LaserGameV3/Blueprints/Old/BP_LaserParent` _lasthitactor))
          (if (and (`KismetSystemLibrary.DoesImplementInterface` _asbp_laser_parent "/Game/Blueprints/LaserMiniGame/LaserGameV3/BPI_Laser.BPI_Laser_C") (`KismetArrayLibrary.Array_IsEmpty` (`/Game/Blueprints/LaserMiniGame/LaserGameV3/Blueprints/Old/BP_LaserParent.LasersAttached` _asbp_laser_parent)))
            (message `/Game/Blueprints/LaserMiniGame/LaserGameV3/BPI_Laser.LaserBounce` (`self.LastHitActor`) self false (struct))
            (else
              (set `/Game/Blueprints/LaserMiniGame/LaserGameV3/Blueprints/Old/BP_LaserParent.Active` false _asbp_laser_parent))))
        (:`else`)))
    (:`then_1`
      (if (`local.Override`)
        (return false)
        (else
          (`self.K2_DestroyActor`)
          (return true))))))

(fn `ChangeColor`
  (bind _returnvalue (`PrimitiveComponent.CreateDynamicMaterialInstance` (`self.Cylinder`) 0 "/Game/Blueprints/LaserMiniGame/LaserGameV3/Materials/M_Laser.M_Laser" "None"))
  (`MaterialInstanceDynamic.SetVectorParameterValue` _returnvalue "Base Color" (`self.LaserColor`)))

(fn `Set End Point`
  (locals (L_Range :type "Float (double-precision)" :default 3000.0) (LocalHitInfo :type "HitResult Structure") (L_HitActor :type "Actor Object Reference"))
  (bind _returnvalue (`self.GetActorUpVector`))
  (bind (_bblockinghit _binitialoverlap _time _distance _location _impactpoint _normal _impactnormal _physmat _hitactor _hitcomponent _hitbonename _bonename _hititem _elementindex _faceindex _tracestart) (`GameplayStatics.BreakHitResult` (`local.LocalHitInfo`)))
  (bind _returnvalue_2 (+ (`self.K2_GetActorLocation`) (* _returnvalue 2.0)))
  (bind _outhit (`KismetSystemLibrary.BoxTraceSingle` _returnvalue_2 (+ _returnvalue_2 (* _returnvalue (`local.L_Range`))) (0.0 0.0 0.0) (struct) "TraceTypeQuery1"))
  (bind _output_get (set `local.LocalHitInfo` _outhit))
  (bind (_bblockinghit_2 _binitialoverlap_2 _time_2 _distance_2 _location_2 _impactpoint_2 _normal_2 _impactnormal_2 _physmat_2 _hitactor_2) (`GameplayStatics.BreakHitResult` _output_get))
  (set `local.L_HitActor` _hitactor_2)
  (`SceneComponent.SetWorldScale3D` (`self.SM_Parent`) (`KismetMathLibrary.MakeVector` 0.05 0.05 (`KismetMathLibrary.SelectFloat` (/ (+ _distance_2 1.0) 100.0) (/ (`local.L_Range`) 100.0) _bblockinghit_2)))
  (`local.L_HitActor`
    (:`then`
      (`|ExecutionSequence`
        (:`then_0`
          (if (== (`self.LastHitActor`) (`local.L_HitActor`))
            (bind _asbp_reflect_laser (cast `/Game/Blueprints/LaserMiniGame/LaserGameV3/Blueprints/Old/BP_ReflectLaser` (`self.LastHitActor`)))
            (`self.K2_SetActorLocation` (`self.BounceLaser`) (`.ImpactPoint` (`GameplayStatics.BreakHitResult` (`local.LocalHitInfo`))) false false)
            (`self.K2_SetActorRotation` (`self.BounceLaser`) (`/Game/Blueprints/LaserMiniGame/LaserGameV3/Blueprints/Old/BP_ReflectLaser.Calculate Rotation` _asbp_reflect_laser _impactpoint _impactnormal _tracestart) false)
            (else
              (`|ExecutionSequence`
                (:`then_0`
                  (if (`KismetSystemLibrary.DoesImplementInterface` (`self.LastHitActor`) "/Game/Blueprints/LaserMiniGame/LaserGameV3/BPI_Laser.BPI_Laser_C")
                    (`/Game/Blueprints/LaserMiniGame/LaserGameV3/Blueprints/Old/BP_LaserSpawn.Remove Following Lasers` (`self.SpawnReference`) self)))
                (:`then_1`
                  (if (`KismetSystemLibrary.DoesImplementInterface` (`local.L_HitActor`) "/Game/Blueprints/LaserMiniGame/LaserGameV3/BPI_Laser.BPI_Laser_C")
                    (bind _newlaser (message `/Game/Blueprints/LaserMiniGame/LaserGameV3/BPI_Laser.LaserBounce` (`self.LastHitActor`) self false (`local.LocalHitInfo`)))
                    (set `self.BounceLaser` _newlaser)))))))
        (:`then_1`
          (set `self.LastHitActor` (`local.L_HitActor`)))))
    (:`else`
      (`|ExecutionSequence`
        (:`then_0`
          (bind _lasthitactor (`self.LastHitActor`)
            (:`then`
              (if (`KismetSystemLibrary.DoesImplementInterface` _lasthitactor "/Game/Blueprints/LaserMiniGame/LaserGameV3/BPI_Laser.BPI_Laser_C")
                (message `/Game/Blueprints/LaserMiniGame/LaserGameV3/BPI_Laser.LaserBounce` (`self.LastHitActor`) self false (`local.LocalHitInfo`))))
            (:`else`)))
        (:`then_1`
          (set `self.LastHitActor` null)
          (set `self.BounceLaser` null))))))

(fn `UpdateID`
  (params (Input_Append :type String))
  (returns (ReturnValue :type String))
  (return (`KismetStringLibrary.Concat_StrStr` (`self.Laser_ID`) Input_Append)))

(fn `UserConstructionScript`
  (`parent.UserConstructionScript`))