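; BP_ReflectLaser is a reflector for the laser minigame that bounces incoming lasers off its surface.
; LaserBounce spawns a BP_LaserChild at the impact point, its Z axis mirrored about the hit normal, inheriting color and a "B"-updated ID.
; Each child registers in LasersAttached and the source's ChildLaser list.
; On a failed hit, it destroys attached lasers whose ID contains the incoming ID, using substring matching to clear descendants.
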(fn `Calculate Rotation`
  (params (`Impact Point` :type "Vector Structure") (`Impact Normal` :type "Vector Structure") (`Trace Start` :type "Vector Structure"))
  (returns (ReturnValue :type "Rotator Structure"))
  (return (`KismetMathLibrary.MakeRotFromZ` (`KismetMathLibrary.MirrorVectorByNormal` (- `Impact Point` `Trace Start`) `Impact Normal`))))

(fn `Clear Attached Lasers`
  (params (`ID Clear` :type String))
  (bind (_arrayindex _arrayelement) (`/Engine/EditorBlueprintResources/StandardMacros.ReverseForEachLoop` (`self.LasersAttached`))
    (:`LoopBody`
      (`/Engine/EditorBlueprintResources/StandardMacros.IsValid` _arrayelement
        (:`Is Valid`
          (if (`KismetStringLibrary.Contains` (`/Game/Blueprints/LaserMiniGame/LaserGameV3/Blueprints/Old/BP_LaserChild.Laser_ID` _arrayelement) (`local.ID Clear`))
            (`self.K2_DestroyActor` _arrayelement)
            (`KismetArrayLibrary.Array_RemoveItem` (`self.LasersAttached`) _arrayelement)))))))

(fn `LaserBounce`
  (params (P_LaserHit :type "/Game/Blueprints/LaserMiniGame/LaserGameV3/Blueprints/Old/BP_LaserChild Object Reference") (P_HitResponce :type Boolean) (P_HitInfo :type "HitResult Structure"))
  (returns (NewLaser :type "/Game/Blueprints/LaserMiniGame/LaserGameV3/Blueprints/Old/BP_LaserChild Object Reference"))
  (bind _p_laserhit (`local.P_LaserHit`))
  (bind (_bblockinghit _binitialoverlap _time _distance _location _impactpoint _normal _impactnormal _physmat _hitactor _hitcomponent _hitbonename _bonename _hititem _elementindex _faceindex _tracestart) (`GameplayStatics.BreakHitResult` (`local.P_HitInfo`)))
  (if (`local.P_HitResponce`)
    (bind _returnvalue (`|SpawnActorFromClass` "/Game/Blueprints/LaserMiniGame/LaserGameV3/Blueprints/Old/BP_LaserChild.BP_LaserChild_C" (`KismetMathLibrary.MakeTransform` _impactpoint (`self.Calculate Rotation` _impactpoint _impactnormal _tracestart)) "Undefined" "MultiplyWithRoot" null (`/Game/Blueprints/LaserMiniGame/LaserGameV3/Blueprints/Old/BP_LaserChild.UpdateID` _p_laserhit "B") (`/Game/Blueprints/LaserMiniGame/LaserGameV3/Blueprints/Old/BP_LaserParent.LaserColor` _p_laserhit) (`/Game/Blueprints/LaserMiniGame/LaserGameV3/Blueprints/Old/BP_LaserParent.SpawnReference` _p_laserhit) null))
    (`KismetArrayLibrary.Array_Add` (`self.LasersAttached`) _returnvalue)
    (`KismetArrayLibrary.Array_Add` (`/Game/Blueprints/LaserMiniGame/LaserGameV3/Blueprints/Old/BP_LaserSpawn.ChildLaser` (`/Game/Blueprints/LaserMiniGame/LaserGameV3/Blueprints/Old/BP_LaserParent.SpawnReference` (`local.P_LaserHit`))) _returnvalue)
    (return _returnvalue)
    (else
      (`self.Clear Attached Lasers` (`/Game/Blueprints/LaserMiniGame/LaserGameV3/Blueprints/Old/BP_LaserChild.Laser_ID` (`local.P_LaserHit`))))))

(fn `UserConstructionScript`
  (`parent.UserConstructionScript`))