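; BP_LaserCube is a laser minigame piece that re-emits an incoming laser along its Arrow's forward direction.
; On a hit while inactive, LaserBounce spawns a BP_LaserChild with the same color and a "C"-updated ID, attached to SMParent.
; The child registers in LasersAttached and the spawn reference's ChildLaser list.
; A lost hit deactivates the cube and calls ClearLaserAttached.
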(fn `LaserBounce`
  (params (P_LaserHit :type "/Game/Blueprints/LaserMiniGame/LaserGameV3/Blueprints/Old/BP_LaserChild Object Reference") (P_HitResponce :type Boolean) (P_HitInfo :type "HitResult Structure"))
  (returns (NewLaser :type "/Game/Blueprints/LaserMiniGame/LaserGameV3/Blueprints/Old/BP_LaserChild Object Reference"))
  (bind _p_laserhit (`local.P_LaserHit`))
  (`/Engine/EditorBlueprintResources/StandardMacros.IsValid` P_LaserHit
    (:`Is Valid`
      (set `self.SpawnReference` (`/Game/Blueprints/LaserMiniGame/LaserGameV3/Blueprints/Old/BP_LaserParent.SpawnReference` P_LaserHit))
      (if (or (and (`local.P_HitResponce`) (not (`self.Active`))) (not (`local.P_HitResponce`)))
        (bind _output_get (set `self.Active` (`local.P_HitResponce`)))
        (if _output_get
          (bind _returnvalue (`|SpawnActorFromClass` "/Game/Blueprints/LaserMiniGame/LaserGameV3/Blueprints/Old/BP_LaserChild.BP_LaserChild_C" (`KismetMathLibrary.MakeTransform` (`SceneComponent.K2_GetComponentLocation` (`self.Arrow`)) (`KismetMathLibrary.MakeRotFromZ` (`SceneComponent.GetForwardVector` (`self.Arrow`)))) "Undefined" "MultiplyWithRoot" null (`/Game/Blueprints/LaserMiniGame/LaserGameV3/Blueprints/Old/BP_LaserChild.UpdateID` _p_laserhit "C") (`/Game/Blueprints/LaserMiniGame/LaserGameV3/Blueprints/Old/BP_LaserParent.LaserColor` _p_laserhit) (`self.SpawnReference`) null))
          (`self.K2_AttachToComponent` _returnvalue (`self.SM_Parent`) "None" "KeepWorld" "KeepWorld" "KeepRelative" false)
          (`KismetArrayLibrary.Array_Add` (`self.LasersAttached`) _returnvalue)
          (`KismetArrayLibrary.Array_Add` (`/Game/Blueprints/LaserMiniGame/LaserGameV3/Blueprints/Old/BP_LaserSpawn.ChildLaser` (`self.SpawnReference`)) _returnvalue)
          (return _returnvalue)
          (else
            (`self.ClearLaserAttached`)))))))

(fn `UserConstructionScript`
  (`parent.UserConstructionScript`))