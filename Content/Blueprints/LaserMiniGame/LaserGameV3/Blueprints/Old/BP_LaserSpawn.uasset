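; Laser emitter actor for the laser minigame that starts a beam and tracks its segments.
; On BeginPlay it spawns a BP_LaserChild at its Arrow, passing its display name as laser ID along with color and spawn reference, and stores it in ChildLaser.
; RemoveFollowingLasers walks that array backwards, calls CancelTargetHit on lasers whose ID contains the given laser's ID, and drops those that return true.
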(event `self.ReceiveBeginPlay`
  (set `self.SpawnLaser` self)
  (set `self.ID` (`KismetSystemLibrary.GetDisplayName` self))
  (bind _returnvalue (`|SpawnActorFromClass` "/Game/Blueprints/LaserMiniGame/LaserGameV3/Blueprints/Old/BP_LaserChild.BP_LaserChild_C" (`KismetMathLibrary.MakeTransform` (`SceneComponent.K2_GetComponentLocation` (`self.Arrow`)) (`self.K2_GetActorRotation`)) "Undefined" "MultiplyWithRoot" null (`self.ID`) (`self.LaserColor`) (`self.SpawnReference`) null))
  (`KismetArrayLibrary.Array_Add` (`self.ChildLaser`) _returnvalue))

(fn `Remove Following Lasers`
  (params (`Laser Reference` :type "/Game/Blueprints/LaserMiniGame/LaserGameV3/Blueprints/Old/BP_LaserChild Object Reference"))
  (locals (`L_ID Remove` :type String))
  (set `local.L_ID Remove` (`/Game/Blueprints/LaserMiniGame/LaserGameV3/Blueprints/Old/BP_LaserChild.Laser_ID` `Laser Reference`))
  (bind (_arrayindex _arrayelement) (`/Engine/EditorBlueprintResources/StandardMacros.ReverseForEachLoop` (`self.ChildLaser`))
    (:`LoopBody`
      (`/Engine/EditorBlueprintResources/StandardMacros.IsValid` _arrayelement
        (:`Is Valid`
          (if (`KismetStringLibrary.Contains` (`/Game/Blueprints/LaserMiniGame/LaserGameV3/Blueprints/Old/BP_LaserChild.Laser_ID` _arrayelement) (`local.L_ID Remove`))
            (bind _remove_from_array (`/Game/Blueprints/LaserMiniGame/LaserGameV3/Blueprints/Old/BP_LaserChild.Cancel Target Hit` _arrayelement (`KismetStringLibrary.EqualEqual_StrStr` (`/Game/Blueprints/LaserMiniGame/LaserGameV3/Blueprints/Old/BP_LaserChild.Laser_ID` _arrayelement) (`local.L_ID Remove`))))
            (if _remove_from_array
              (`KismetArrayLibrary.Array_RemoveItem` (`self.ChildLaser`) _arrayelement))))))))

(fn `UserConstructionScript`
  (`parent.UserConstructionScript`))