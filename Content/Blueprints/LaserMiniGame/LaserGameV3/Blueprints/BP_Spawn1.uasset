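; BP_Spawn1 is a laser spawn Blueprint in the laser mini-game that exposes on and off controls for a laser.
; On BeginPlay it prints a debug message and deactivates the laser on its BPSEmitter, so the laser starts off.
; TurnOnLaser only forwards activation to BPCHandler, while TurnOffLaser deactivates the emitter directly and then notifies the handler.
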(event `self.ReceiveBeginPlay`
  (`KismetSystemLibrary.PrintString` "APAGADO")
  (`/Game/Blueprints/LaserMiniGame/LaserGameV3/Blueprints/BuildingBlocks/BPS_Emitter.DeactivateLaser` (`self.BPS_Emitter`)))

(fn `TurnOffLaser`
  (`/Game/Blueprints/LaserMiniGame/LaserGameV3/Blueprints/BuildingBlocks/BPS_Emitter.DeactivateLaser` (`self.BPS_Emitter`))
  (`/Game/Blueprints/LaserMiniGame/LaserGameV3/Blueprints/BuildingBlocks/BPC_Handler.DeactivateHandler` (`self.BPC_Handler`) null))

(fn `TurnOnLaser`
  (`/Game/Blueprints/LaserMiniGame/LaserGameV3/Blueprints/BuildingBlocks/BPC_Handler.ActivateHandler` (`self.BPC_Handler`) null))

(fn `UserConstructionScript`)