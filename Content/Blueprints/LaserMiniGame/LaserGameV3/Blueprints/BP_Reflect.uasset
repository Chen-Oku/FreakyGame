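; BP_Reflect is a rotatable reflector piece for the laser minigame, turned by player interaction.
; StartInteract steps its yaw, or its pitch when VerticalRotation is set, provided rotation is allowed and none is running.
; AngleTrack accumulates the steps, reversing direction whenever the next would leave zero to AngleRange.
; A timeline lerps the actor along the shortest path, while CanReceiveLaser always returns false.
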(event `/Game/Blueprints/LaserMiniGame/BPI_FreakInteract.StartInteract`
  (bind _returnvalue (+ (`self.AngleTrack`) (`self.VertRotationAngle`)))
  (bind _returnvalue_2 (+ (`self.AngleTrack`) (`self.HorRotationAngle`)))
  ; Interact and H/V-Rotation
  (if (and (`self.bCanRotate`) (not (`self.bIsRotating`)))
    (bind _output_get (set `self.InicialRotation` (`self.K2_GetActorRotation`)))
    (if (`self.bVerticalRotation`)
      (if (or (> _returnvalue (`self.AngleRange`)) (< _returnvalue 0.0))
        (set `self.VertRotationAngle` (* (`self.VertRotationAngle`) -1.0)))
      (set `self.TargetRotation` (`KismetMathLibrary.MakeRotator` (.roll (`self.InicialRotation`)) (+ (.pitch (`self.InicialRotation`)) (`self.VertRotationAngle`)) (.yaw (`self.InicialRotation`))))
      (set `self.AngleTrack` _returnvalue)
      (else
        (if (or (> _returnvalue_2 (`self.AngleRange`)) (< _returnvalue_2 0.0))
          (set `self.HorRotationAngle` (* (`self.HorRotationAngle`) -1.0)))
        (bind _output_get_2 (set `self.TargetRotation` (`KismetMathLibrary.ComposeRotators` (`self.K2_GetActorRotation`) (`KismetMathLibrary.MakeRotator` 0.0 0.0 (`self.HorRotationAngle`)))))
        (set `self.AngleTrack` _returnvalue_2)))
    (set `self.bIsRotating` true)
    (bind (_direction _rotacionanim) (`Timeline|Timeline` :`NewTime` 5.0 :!via `PlayFromStart`)
      (:`Update`
        (`self.K2_SetActorRotation` (`KismetMathLibrary.RLerp` _output_get _output_get_2 _rotacionanim true)))
      (:`Finished`
        (set `self.bIsRotating` false)))))

(fn `CanReceiveLaser?`
  (returns (bCanReceive :type Boolean))
  (return false))

(fn `UserConstructionScript`)