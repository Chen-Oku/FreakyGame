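; Rotatable mirror for the laser minigame that turns one angle step per interaction and always reports it can receive the laser.
; Each step is either pitch or yaw, depending on VerticalRotation, and a tracked angle flips the step direction at the range limits, producing a back-and-forth sweep.
; A timeline lerps the actor to the target rotation along the shortest path, ignoring new interactions until it finishes.
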(event `self.StartInteract`
  (bind _returnvalue (+ (`self.AngleTrack`) (`self.VertRotationAngle`)))
  (bind _returnvalue_2 (+ (`self.AngleTrack`) (`self.HorRotationAngle`)))
  ; Interact and H/V-Rotation
  (if (and (`self.bCanRotate`) (not (`self.bIsRotating`)))
    (bind _output_get (set `self.InicialRotation` (`self.K2_GetActorRotation`)))
    (if (`self.bVerticalRotation`)
      (if (or (> _returnvalue (`self.AngleRange`)) (< _returnvalue 0.0))
        (set `self.VertRotationAngle` (* (`self.VertRotationAngle`) -1.0)))
      (set `self.TargetRotation` (`KismetMathLibrary.MakeRotator` (.roll (`self.InicialRotation`)) (+ (.pitch (`self.InicialRotation`)) (`self.VertRotationAngle`)) (.yaw (`self.InicialRotation`))))
      (set `self.AngleTrack` _returnvalue)
      (else
        (if (or (> _returnvalue_2 (`self.AngleRange`)) (< _returnvalue_2 0.0))
          (set `self.HorRotationAngle` (* (`self.HorRotationAngle`) -1.0)))
        (bind _output_get_2 (set `self.TargetRotation` (`KismetMathLibrary.ComposeRotators` (`self.K2_GetActorRotation`) (`KismetMathLibrary.MakeRotator` 0.0 0.0 (`self.HorRotationAngle`)))))
        (set `self.AngleTrack` _returnvalue_2)))
    (set `self.bIsRotating` true)
    (bind (_direction _rotacionanim) (`Timeline|RotacionEspejo` :`NewTime` 5.0 :!via `PlayFromStart`)
      (:`Update`
        (`self.K2_SetActorRotation` (`KismetMathLibrary.RLerp` _output_get _output_get_2 _rotacionanim true)))
      (:`Finished`
        (set `self.bIsRotating` false)))))

(fn `CanReceiveLaser?`
  (returns (bCanReceive :type Boolean))
  (return true))

(fn `PlayPushAnim`
  (returns (TrueIfAnim :type Boolean))
  (return true))

(fn `UserConstructionScript`)